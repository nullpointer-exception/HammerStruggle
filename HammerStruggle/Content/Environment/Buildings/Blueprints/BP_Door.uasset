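; Double-door building actor that swings two door meshes open or closed according to an OpenDoor flag set through ToggelDoors.
; Tick applies relative rotations to both leaves each frame, using a Rotation helper fed target angles and delta time.
; A Room overlap volume counts actors inside to maintain IsEmpty, which is only debug-printed and does not drive the doors.
; Construction caches the Scene component's world transform as SpawnLocation.
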(event `self.ReceiveTick`
  (params (DeltaSeconds :type "Float (single-precision)"))
  (if (`self.OpenDoor`)
    (`self.OpenDoors` DeltaSeconds)
    (else
      (`self.CloseDoors` DeltaSeconds)))
  (`KismetSystemLibrary.PrintString` (`KismetStringLibrary.Conv_BoolToString` (`self.IsEmpty`)) true true (struct :`G` 0.66 :`B` 1.0 :`A` 1.0) DeltaSeconds))

(event `self.Room.OnComponentBeginOverlap`
  (params (OverlappedComponent :type "PrimitiveComponent Object Reference") (OtherActor :type "Actor Object Reference") (OtherComp :type "PrimitiveComponent Object Reference") (OtherBodyIndex :type Integer) (bFromSweep :type Boolean) (SweepResult :type "HitResult Structure (by ref)"))
  (`/Engine/EditorBlueprintResources/StandardMacros.IncrementInt` (`self.ActorsInside`)
    (:`  `
      (set `self.IsEmpty` false))))

(event `self.Room.OnComponentEndOverlap`
  (params (OverlappedComponent :type "PrimitiveComponent Object Reference") (OtherActor :type "Actor Object Reference") (OtherComp :type "PrimitiveComponent Object Reference") (OtherBodyIndex :type Integer))
  (bind _result (`/Engine/EditorBlueprintResources/StandardMacros.DecrementInt` (`self.ActorsInside`))
    (:`  `
      (if (<= _result 0)
        (set `self.IsEmpty` true)))))

(fn `CloseDoors`
  (params (DeltaTime :type "Float (double-precision)"))
  (bind _sm_door_left (`self.SM_Door_Left`))
  (bind _sm_door_right (`self.SM_Door_Right`))
  (`SceneComponent.K2_SetRelativeRotation` _sm_door_left (`self.Rotation` _sm_door_left (struct :`Yaw` 180.0) DeltaTime) false false)
  (`SceneComponent.K2_SetRelativeRotation` _sm_door_right (`self.Rotation` _sm_door_right (struct :`Yaw` 180.0) DeltaTime) false false))

(fn `OpenDoors`
  (params (DeltaTime :type "Float (double-precision)"))
  (bind _sm_door_right (`self.SM_Door_Right`))
  (bind _sm_door_left (`self.SM_Door_Left`))
  (`SceneComponent.K2_SetRelativeRotation` _sm_door_right (`self.Rotation` _sm_door_right (struct :`Yaw` 270.0) DeltaTime) false false)
  (`SceneComponent.K2_SetRelativeRotation` _sm_door_left (`self.Rotation` _sm_door_left (struct :`Yaw` 90.0) DeltaTime) false false))

(fn `ToggelDoors`
  (params (`Open?` :type Boolean))
  (if `Open?`
    (set `self.OpenDoor` true)
    (else
      (set `self.OpenDoor` false))))

(fn `UserConstructionScript`
  (set `self.SpawnLocation` (`SceneComponent.K2_GetComponentToWorld` (`self.Scene`))))