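; Blacksmith building that serves as the player's between-rounds area, with a room overlap volume and two swinging doors.
; Entering switches the player's weapon and shield attachment, adds round resources and ends the round through RoundController.
; Leaving switches attachment back, adds resources again, then after a short delay sets doors open and starts the round unless re-entered.
; Tick drives both doors' rotation from the OpenDoor flag.
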(event `self.Room.OnComponentBeginOverlap`
  (params (OverlappedComponent :type "PrimitiveComponent Object Reference") (OtherActor :type "Actor Object Reference") (OtherComp :type "PrimitiveComponent Object Reference") (OtherBodyIndex :type Integer) (bFromSweep :type Boolean) (SweepResult :type "HitResult Structure (by ref)"))
  ;[1 1 1] Change Weapon and Shield attachment
  ;;[0.5885 1 0.5795] Idle
  (`self.ChangeAttachment` OtherActor true)
  (set `self.IsPlayerInside` true)
  (bind _asbp_hsplayer (cast `/Game/Characters/PC/Blueprints/BP_HSPlayer` OtherActor))
  (`/Game/Characters/PC/Blueprints/BP_HSPlayer.OnRoundEnd` _asbp_hsplayer)
  (`/Game/Gameplay/Round/BP_RoundController.EndRound` (`self.RoundController`)))

(event `self.Room.OnComponentEndOverlap`
  (params (OverlappedComponent :type "PrimitiveComponent Object Reference") (OtherActor :type "Actor Object Reference") (OtherComp :type "PrimitiveComponent Object Reference") (OtherBodyIndex :type Integer))
  ;[1 1 1] Change Weapon and Shield attachment
  ;;[1 0.561 0.5072] Fighting
  (`self.ChangeAttachment` OtherActor)
  (set `self.IsPlayerInside` false)
  (`KismetSystemLibrary.Delay` 1.5)
  (`self.ToggelDoors` true)
  (if (not (`self.IsPlayerInside`))
    (`/Game/Gameplay/Round/BP_RoundController.StartRound` (`self.RoundController`))))

(event `self.ReceiveTick`
  (params (DeltaSeconds :type "Float (single-precision)"))
  (if (`self.OpenDoor`)
    (`self.OpenDoors` DeltaSeconds)
    (else
      (`self.CloseDoors` DeltaSeconds))))

(fn `ChangeAttachment`
  (params (Object :type "Actor Object Reference") (IsBlacksmith :type Boolean))
  (bind _asbp_hsplayer (cast `/Game/Characters/PC/Blueprints/BP_HSPlayer` Object))
  (`HSPlayer.ChangeAttachment` _asbp_hsplayer IsBlacksmith)
  (set `/Game/Characters/PC/Blueprints/BP_HSPlayer.InBlacksmith` IsBlacksmith _asbp_hsplayer)
  (`/Game/Characters/PC/Blueprints/BP_HSPlayer.AddRoundRessourcesToAll` _asbp_hsplayer))

(fn `CloseDoors`
  (params (DeltaTime :type "Float (double-precision)"))
  (bind _sm_door_left (`self.SM_Door_Left`))
  (bind _sm_door_right (`self.SM_Door_Right`))
  (`SceneComponent.K2_SetRelativeRotation` _sm_door_left (`self.Rotation` _sm_door_left (struct :`Yaw` 180.0) DeltaTime) false false)
  (`SceneComponent.K2_SetRelativeRotation` _sm_door_right (`self.Rotation` _sm_door_right (struct :`Yaw` 180.0) DeltaTime) false false))

(fn `OpenDoors`
  (params (DeltaTime :type "Float (double-precision)"))
  (bind _sm_door_right (`self.SM_Door_Right`))
  (bind _sm_door_left (`self.SM_Door_Left`))
  (`SceneComponent.K2_SetRelativeRotation` _sm_door_right (`self.Rotation` _sm_door_right (struct :`Yaw` 270.0) DeltaTime) false false)
  (`SceneComponent.K2_SetRelativeRotation` _sm_door_left (`self.Rotation` _sm_door_left (struct :`Yaw` 90.0) DeltaTime) false false))

(fn `ToggelDoors`
  (params (`Open?` :type Boolean))
  (if `Open?`
    (set `self.OpenDoor` true)
    (else
      (set `self.OpenDoor` false))))

(fn `UserConstructionScript`)