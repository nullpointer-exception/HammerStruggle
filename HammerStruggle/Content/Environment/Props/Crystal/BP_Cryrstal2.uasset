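; BP_Cryrstal2 is a crystal prop that hovers up and down while spinning around its yaw axis.
; The construction script caches the spawn position as the hover anchor.
; Tick advances a timer whose degree-based sine drives an unclamped vertical lerp between offsets above and below that anchor, so negative sine values overshoot the upper point.
; Tick also adds frame-scaled yaw to the actor's rotation.
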(event `self.ReceiveTick`
  (params (DeltaSeconds :type "Float (single-precision)"))
  (bind _sceneroot (`self.SceneRoot`))
  (bind (_spawnpos_x _spawnpos_y _spawnpos_z) (`KismetMathLibrary.BreakVector` (`self.SpawnPos`)))
  (bind _offsetz (`self.OffsetZ`))
  ;[1 1 1] HoverEffect
  (bind _output_get (set `self.SinTimer` (+ (* DeltaSeconds (`self.SpeedHover`)) (`self.SinTimer`))))
  (`SceneComponent.K2_SetWorldLocation` _sceneroot (`KismetMathLibrary.VLerp` (`KismetMathLibrary.MakeVector` _spawnpos_x _spawnpos_y (+ _spawnpos_z _offsetz)) (`KismetMathLibrary.MakeVector` _spawnpos_x _spawnpos_y (- _spawnpos_z _offsetz)) (`KismetMathLibrary.DegSin` _output_get)) false false)
  (`SceneComponent.K2_SetWorldRotation` _sceneroot (`KismetMathLibrary.MakeRotator` (.roll (`self.K2_GetActorRotation`)) (.pitch (`self.K2_GetActorRotation`)) (+ (.yaw (`self.K2_GetActorRotation`)) (* DeltaSeconds (`self.RotationSpeed`)))) false false))

(fn `UserConstructionScript`
  (set `self.SpawnPos` (`self.K2_GetActorLocation`)))