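; AI thrower character that launches a projectile at BP_HSPlayer along a computed ballistic arc.
; ThrowProjectileFunc solves the launch-angle equation from its Velocity and Gravity variables and the horizontal and vertical offset to the player.
; It spawns the Projectile at its own location, yawed toward the player and pitched at the smaller of the two solutions.
; A negative discriminant prints an unreachable message instead of throwing.
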(fn `ThrowProjectileFunc`
  (bind (_returnvalue_x _returnvalue_y _returnvalue_z) (`KismetMathLibrary.BreakVector` (`self.K2_GetActorLocation`)))
  (bind _returnvalue (`self.K2_GetActorLocation`))
  (bind _gravity (`self.Gravity`))
  (bind _returnvalue_2 (`KismetMathLibrary.Square` (`self.Velocity`)))
  (bind _outactors (`GameplayStatics.GetAllActorsOfClass` "/Game/Characters/Player/Blueprints/BP_HSPlayer.BP_HSPlayer_C"))
  (for _array_element _outactors
    _)
  (bind (_returnvalue_x_2 _returnvalue_y_2 _returnvalue_z_2) (`KismetMathLibrary.BreakVector` (`self.K2_GetActorLocation` _array_element)))
  (bind _returnvalue_3 (`KismetMathLibrary.VSize2D` (`KismetMathLibrary.MakeVector2D` (- _returnvalue_x_2 _returnvalue_x) (- _returnvalue_y_2 _returnvalue_y))))
  (bind _returnvalue_4 (- (`KismetMathLibrary.Square` _returnvalue_2) (* _gravity (+ (* (`KismetMathLibrary.Square` _returnvalue_3) _gravity) (* (* (- _returnvalue_z_2 _returnvalue_z) _returnvalue_2) 2.0)))))
  (if (>= _returnvalue_4 0.0)
    (bind (_returnvalue_roll _returnvalue_pitch _returnvalue_yaw) (`KismetMathLibrary.BreakRotator` (`KismetMathLibrary.FindLookAtRotation` _returnvalue (`self.K2_GetActorLocation` _array_element))))
    (bind _returnvalue_5 (`KismetMathLibrary.Sqrt` _returnvalue_4))
    (bind _returnvalue_6 (* _returnvalue_3 _gravity))
    (`|SpawnActorFromClass` "/Game/Characters/KI/Projectile.Projectile_C" (`KismetMathLibrary.MakeTransform` _returnvalue (`KismetMathLibrary.MakeRotator` _returnvalue_roll (`KismetMathLibrary.FMin` (`KismetMathLibrary.DegAtan` (/ (- _returnvalue_2 _returnvalue_5) _returnvalue_6)) (`KismetMathLibrary.DegAtan` (/ (+ _returnvalue_5 _returnvalue_2) _returnvalue_6))) _returnvalue_yaw)) "Undefined" "OverrideRootScale" null null)
    (else
      (`KismetSystemLibrary.PrintString` "Unreachabel"))))

(fn `UserConstructionScript`)