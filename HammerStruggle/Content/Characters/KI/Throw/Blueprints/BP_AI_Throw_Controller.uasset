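; AI controller for the throwing enemy, running the BT_Throw behavior tree when it possesses a BP_AIBase character.
; Perception updates on a BP_HSPlayer write CanSeePlayer and the Player object to the blackboard.
; Tick writes the distance between the AI character and player pawn 0 to DistanceToPlayer every frame.
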(event `self.ReceiveTick`
  (params (DeltaSeconds :type "Float (single-precision)"))
  (`BlackboardComponent.SetValueAsFloat` (`AIBlueprintHelperLibrary.GetBlackboard` null) "DistanceToPlayer" (`KismetMathLibrary.VSize` (- (`self.K2_GetActorLocation` (`GameplayStatics.GetPlayerPawn` 0)) (`self.K2_GetActorLocation` (`self.AICharacter`))))))

(event `self.ReceivePossess`
  (params (PossessedPawn :type "Pawn Object Reference"))
  (bind _asbp_aibase (cast `/Game/Characters/KI/BP_AIBase` PossessedPawn))
  (set `self.AICharacter` _asbp_aibase)
  (`self.RunBehaviorTree` "/Game/Characters/KI/Throw/BB_BT/BT_Throw.BT_Throw"))

(event `self.AIPerception.OnTargetPerceptionUpdated`
  (params (Actor :type "Actor Object Reference") (Stimulus :type "AIStimulus Structure"))
  (bind _returnvalue (`AIBlueprintHelperLibrary.GetBlackboard` null))
  (bind _asbp_hsplayer (cast `/Game/Characters/Player/Blueprints/BP_HSPlayer` Actor))
  (`BlackboardComponent.SetValueAsBool` _returnvalue "CanSeePlayer" (`.bSuccessfullySensed` (break `AIStimulus` Stimulus)))
  (`BlackboardComponent.SetValueAsObject` _returnvalue "Player" _asbp_hsplayer))

(fn `UserConstructionScript`)