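; Throwing enemy AI character whose Throw function lobs a projectile at the player.
; Throw solves the ballistic equation from Velocity, Gravity and the player's Z-offset position, printing a debug message if the target is unreachable.
; Otherwise it spawns the projectile at the Scene component, yawed toward the player and pitched at the lower launch angle, then passes it DamageThrow.
; The event graph is empty, so Throw is not triggered here.
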(fn `Throw`
  (locals (ZOffset :type "Float (double-precision)" :default -50.0) (Gravity :type "Float (double-precision)" :default 980.0) (Velocity :type "Float (double-precision)" :default 2000.0))
  (bind _returnvalue (`GameplayStatics.GetPlayerPawn` 0))
  (bind _gravity (`local.Gravity`))
  (bind _returnvalue_2 (`KismetMathLibrary.Square` (`local.Velocity`)))
  (bind _returnvalue_3 (`SceneComponent.K2_GetComponentLocation` (`self.Scene`)))
  (bind (_returnvalue_x _returnvalue_y _returnvalue_z) (`KismetMathLibrary.BreakVector` (`SceneComponent.K2_GetComponentLocation` (`self.Scene`))))
  (bind (_returnvalue_x_2 _returnvalue_y_2 _returnvalue_z_2) (`KismetMathLibrary.BreakVector` (`self.K2_GetActorLocation` _returnvalue)))
  (bind _returnvalue_4 (`KismetMathLibrary.VSize2D` (`KismetMathLibrary.MakeVector2D` (- _returnvalue_x_2 _returnvalue_x) (- _returnvalue_y_2 _returnvalue_y))))
  (bind _returnvalue_5 (* _returnvalue_4 _gravity))
  (bind _returnvalue_6 (- (`KismetMathLibrary.Square` _returnvalue_2) (* _gravity (+ (* (`KismetMathLibrary.Square` _returnvalue_4) _gravity) (* (* (- (- _returnvalue_z_2 (`local.ZOffset`)) _returnvalue_z) _returnvalue_2) 2.0)))))
  (bind _returnvalue_7 (`KismetMathLibrary.Sqrt` _returnvalue_6))
  (bind _asbp_hsplayer (cast `/Game/Characters/PC/Blueprints/BP_HSPlayer` _returnvalue))
  (if (>= _returnvalue_6 0.0)
    (bind (_returnvalue_x_3 _returnvalue_y_3 _returnvalue_z_3) (`KismetMathLibrary.BreakVector` (`self.K2_GetActorLocation` _asbp_hsplayer)))
    (bind (_returnvalue_roll _returnvalue_pitch _returnvalue_yaw) (`KismetMathLibrary.BreakRotator` (`KismetMathLibrary.FindLookAtRotation` _returnvalue_3 (`KismetMathLibrary.MakeVector` _returnvalue_x_3 _returnvalue_y_3 (- _returnvalue_z_3 (`local.ZOffset`))))))
    (bind _returnvalue_8 (`|SpawnActorFromClass` "/Game/Characters/NPC/Enemies/KI/Projectile.Projectile_C" (`KismetMathLibrary.MakeTransform` _returnvalue_3 (`KismetMathLibrary.MakeRotator` _returnvalue_roll (`KismetMathLibrary.FMin` (`KismetMathLibrary.DegAtan` (/ (- _returnvalue_2 _returnvalue_7) _returnvalue_5)) (`KismetMathLibrary.DegAtan` (/ (+ _returnvalue_7 _returnvalue_2) _returnvalue_5))) _returnvalue_yaw)) "DontSpawnIfColliding" "OverrideRootScale" null null))
    (`/Engine/EditorBlueprintResources/StandardMacros.IsValid` _returnvalue_8
      (:`Is Valid`
        (set `/Game/Characters/NPC/Enemies/KI/Projectile.Damage` (`self.DamageThrow`) _returnvalue_8)))
    (else
      (`KismetSystemLibrary.PrintString` "Unreachabel"))))

(fn `UserConstructionScript`
  (`parent.UserConstructionScript`))