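; Base AI enemy character that tracks health, shows a camera-facing health bar widget and drops resources on death.
; Any damage lowers health; at zero it stops the AI brain, waits for the animation, then sinks the mesh.
; It then spawns its resource class, optionally spawns a load chest built from LoadRessource, and destroys itself.
; Setter functions assign both resource values.
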(event `self.ReceiveTick`
  (params (DeltaSeconds :type "Float (single-precision)"))
  (bind _widget (`self.Widget`))
  ;[1 1 1] Rotate Widget to Player
  (`SceneComponent.K2_SetWorldRotation` _widget (`KismetMathLibrary.FindLookAtRotation` (`SceneComponent.K2_GetComponentLocation` _widget) (`PlayerCameraManager.GetCameraLocation` (`GameplayStatics.GetPlayerCameraManager` 0))) false false))

(event `self.ReceiveBeginPlay`
  ;[1 1 1] Create Widget
  (bind _asui_aihealth_bar (cast `/Game/Characters/NPC/Enemies/KI/UI_AIHealthBar` (`WidgetComponent.GetUserWidgetObject` (`self.Widget`))))
  (set `/Game/Characters/NPC/Enemies/KI/UI_AIHealthBar.Owner` self _asui_aihealth_bar))

(event `self.ReceiveAnyDamage`
  (params (Damage :type "Float (single-precision)") (DamageType :type "DamageType Object Reference") (InstigatedBy :type "Controller Object Reference") (DamageCauser :type "Actor Object Reference"))
  ;[1 1 1] GetDamage
  (bind _output_get (set `self.Health` (- (`self.Health`) Damage)))
  (if (<= _output_get 0.0)
    (set `self.Health` 0.0)
    (`self.Die`)))

(event `Die`
  (bind _returnvalue (`self.GetTransform`))
  (bind _skeletalmesh (`self.SkeletalMesh`))
  (bind _loadressource (`self.LoadRessource`))
  (bind _returnvalue_2 (`AIBlueprintHelperLibrary.GetAIController` self))
  (bind (_relativelocation_x _relativelocation_y _relativelocation_z) (`KismetMathLibrary.BreakVector` (`SceneComponent.RelativeLocation` _skeletalmesh)))
  ;[1 1 1] Die
  (`/Engine/EditorBlueprintResources/StandardMacros.IsValid` _returnvalue_2
    (:`Is Valid`
      (`AIController.K2_ClearFocus` _returnvalue_2)
      (set `self.IsDead` true)
      (`BrainComponent.StopLogic` (`AIController.BrainComponent` (`AIBlueprintHelperLibrary.GetAIController` self)) "")
      (`KismetSystemLibrary.Delay` 2.0) ; Wait for Anim to End
      (`KismetSystemLibrary.MoveComponentTo` _skeletalmesh (`KismetMathLibrary.MakeVector` _relativelocation_x _relativelocation_y (- _relativelocation_z 100.0)) (`SceneComponent.RelativeRotation` _skeletalmesh) false false 2.0)
      (`|SpawnActorFromClass` (`self.Ressource`) (`KismetMathLibrary.MakeTransform` (`KismetMathLibrary.MakeVector` (.x (.location _returnvalue)) (.y (.location _returnvalue))) (.rotation _returnvalue) (.scale _returnvalue)) "Undefined" "OverrideRootScale" null null)
      (if (!= _loadressource null)
        (bind _returnvalue_3 (`|SpawnActorFromClass` "/Game/Gameplay/Resources/BP_Ressource_Base_LoadChest.BP_Ressource_Base_LoadChest_C" (`KismetMathLibrary.MakeTransform` (0.0 0.0 0.0)) "Undefined" "OverrideRootScale" null null))
        (`/Game/Gameplay/Resources/BP_Ressource_Base_LoadChest.CreateChest` _returnvalue_3 _loadressource))
      (`self.K2_DestroyActor`))))

(fn `SetLoadRessource`
  (params (Ressource :type "/Game/Gameplay/Resources/Ressources/BP_BaseResouces Class Reference"))
  (set `self.LoadRessource` Ressource))

(fn `SetRessource`
  (params (Ressource :type "/Game/Gameplay/Resources/Ressources/BP_BaseResouces Class Reference"))
  (set `self.Ressource` Ressource))

(fn `UserConstructionScript`)