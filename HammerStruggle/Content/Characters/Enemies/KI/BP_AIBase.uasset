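; BP_AIBase is an enemy AI base with health, a health bar widget and a resource drop on death.
; BeginPlay hands itself to the health bar widget as owner, and Tick turns that widget toward the player camera.
; Damage applies only while the mesh is not animating, then plays ThirdPersonWalk once, so hits during playback are ignored.
; At zero health it spawns NextRessource at its transform and destroys itself.
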(event `self.ReceiveTick`
  (params (DeltaSeconds :type "Float (single-precision)"))
  (bind _widget (`self.Widget`))
  ;[1 1 1] Rotate Widget to Player
  (`SceneComponent.K2_SetWorldRotation` _widget (`KismetMathLibrary.FindLookAtRotation` (`SceneComponent.K2_GetComponentLocation` _widget) (`PlayerCameraManager.GetCameraLocation` (`GameplayStatics.GetPlayerCameraManager` 0))) false false))

(event `self.ReceiveBeginPlay`
  ;[1 1 1] Create Widget
  (bind _asui_aihealth_bar (cast `/Game/Characters/Enemies/KI/UI_AIHealthBar` (`WidgetComponent.GetUserWidgetObject` (`self.Widget`))))
  (set `/Game/Characters/Enemies/KI/UI_AIHealthBar.Owner` self _asui_aihealth_bar))

(event `self.ReceiveAnyDamage`
  (params (Damage :type "Float (single-precision)") (DamageType :type "DamageType Object Reference") (InstigatedBy :type "Controller Object Reference") (DamageCauser :type "Actor Object Reference"))
  (bind _mesh (`self.Mesh`))
  ;[1 1 1] GetDamage
  (if (not (`SkeletalMeshComponent.IsPlaying` _mesh))
    (`SkeletalMeshComponent.PlayAnimation` _mesh "/Game/Characters/Player/Animations/XXX_UE4_Kann_Der_Weg_XXX/ThirdPersonWalk.ThirdPersonWalk" false)
    (bind _output_get (set `self.Health` (- (`self.Health`) Damage)))
    (if (<= _output_get 0.0)
      (`self.Die`))))

(event `Die`
  ;[1 1 1] Die
  (`|SpawnActorFromClass` (`self.NextRessource`) (`self.GetTransform`) "Undefined" "OverrideRootScale" null null)
  (`self.K2_DestroyActor`))

(fn `UserConstructionScript`)