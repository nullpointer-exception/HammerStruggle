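; Throwing AI enemy character whose Throw function launches a projectile at a BP_HSPlayer along a ballistic arc.
; It loops over all players with an empty body, so the aim uses the last one found, lowered by ZOffset.
; The closed-form trajectory equation takes Velocity and Gravity and picks the lower of two launch pitches, with yaw from look-at rotation.
; A negative discriminant means out of range, so it only prints a message.
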(fn `Throw`
  (bind _gravity (`self.Gravity`))
  (bind _returnvalue (`KismetMathLibrary.Square` (`self.Velocity`)))
  (bind _returnvalue_2 (`SceneComponent.K2_GetComponentLocation` (`self.Scene`)))
  (bind (_returnvalue_x _returnvalue_y _returnvalue_z) (`KismetMathLibrary.BreakVector` (`SceneComponent.K2_GetComponentLocation` (`self.Scene`))))
  (bind _outactors (`GameplayStatics.GetAllActorsOfClass` "/Game/Characters/Player/Blueprints/BP_HSPlayer.BP_HSPlayer_C"))
  (for _array_element _outactors
    _)
  (bind (_returnvalue_x_2 _returnvalue_y_2 _returnvalue_z_2) (`KismetMathLibrary.BreakVector` (`self.K2_GetActorLocation` _array_element)))
  (bind _returnvalue_3 (`KismetMathLibrary.VSize2D` (`KismetMathLibrary.MakeVector2D` (- _returnvalue_x_2 _returnvalue_x) (- _returnvalue_y_2 _returnvalue_y))))
  (bind _returnvalue_4 (- (`KismetMathLibrary.Square` _returnvalue) (* _gravity (+ (* (`KismetMathLibrary.Square` _returnvalue_3) _gravity) (* (* (- (- _returnvalue_z_2 (`self.ZOffset`)) _returnvalue_z) _returnvalue) 2.0)))))
  (if (>= _returnvalue_4 0.0)
    (bind (_returnvalue_x_3 _returnvalue_y_3 _returnvalue_z_3) (`KismetMathLibrary.BreakVector` (`self.K2_GetActorLocation` _array_element)))
    (bind (_returnvalue_roll _returnvalue_pitch _returnvalue_yaw) (`KismetMathLibrary.BreakRotator` (`KismetMathLibrary.FindLookAtRotation` _returnvalue_2 (`KismetMathLibrary.MakeVector` _returnvalue_x_3 _returnvalue_y_3 (- _returnvalue_z_3 (`self.ZOffset`))))))
    (bind _returnvalue_5 (`KismetMathLibrary.Sqrt` _returnvalue_4))
    (bind _returnvalue_6 (* _returnvalue_3 _gravity))
    (`|SpawnActorFromClass` "/Game/Characters/Enemies/KI/Projectile.Projectile_C" (`KismetMathLibrary.MakeTransform` _returnvalue_2 (`KismetMathLibrary.MakeRotator` _returnvalue_roll (`KismetMathLibrary.FMin` (`KismetMathLibrary.DegAtan` (/ (- _returnvalue _returnvalue_5) _returnvalue_6)) (`KismetMathLibrary.DegAtan` (/ (+ _returnvalue_5 _returnvalue) _returnvalue_6))) _returnvalue_yaw)) "Undefined" "OverrideRootScale" null null)
    (else
      (`KismetSystemLibrary.PrintString` "Unreachabel"))))

(fn `UserConstructionScript`)