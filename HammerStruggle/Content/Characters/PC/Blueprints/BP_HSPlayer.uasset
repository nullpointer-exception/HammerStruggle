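; Player character with health, stamina and mana, handling movement, pause menu and hammer upgrades that swap modular meshes.
; Attack inputs spend mana or stamina and set attack state outside the blacksmith; stamina regenerates on Tick.
; Capsule overlaps collect resources into a per-round tally, banked at round end, and flag crystal, chest or anvil proximity.
; Interact opens those stations' UIs, locking movement until closed; death only removes the HUD and prints.
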(event `self.Capsule.OnComponentEndOverlap`
  (params (OverlappedComponent :type "PrimitiveComponent Object Reference") (OtherActor :type "Actor Object Reference") (OtherComp :type "PrimitiveComponent Object Reference") (OtherBodyIndex :type Integer))
  ;[1 1 1] Set location Bools to false
  (`|ExecutionSequence`
    (:`then_0`
      (cast `/Game/Gameplay/Crystal/BP_Crystall` OtherActor)
      (cast `BoxComponent` OtherComp)
      (set `self.AtWell` false))
    (:`then_1`
      (cast `/Game/Gameplay/Chest/BP_Chest` OtherActor)
      (cast `BoxComponent` OtherComp)
      (set `self.AtChest` false))
    (:`then_2`
      (cast `/Game/Gameplay/Anvil/BP_Anvil` OtherActor)
      (cast `BoxComponent` OtherComp)
      (set `self.AtAnvil` false))))

(event `self.Capsule.OnComponentBeginOverlap`
  (params (OverlappedComponent :type "PrimitiveComponent Object Reference") (OtherActor :type "Actor Object Reference") (OtherComp :type "PrimitiveComponent Object Reference") (OtherBodyIndex :type Integer) (bFromSweep :type Boolean) (SweepResult :type "HitResult Structure (by ref)"))
  ;[1 1 1] Set Location Bools to True
  (`|ExecutionSequence`
    (:`then_0`
      ;;[1 1 1] Pick Up Ressources
      (bind _asbp_base_resouces (cast `/Game/Gameplay/Resources/Ressources/BP_BaseResouces` OtherActor))
      (`self.AddRessourcesRound` (`|MakeArray` _asbp_base_resouces)))
    (:`then_1`
      ;;[1 1 1] Set AtWell
      (bind _asbp_crystall (cast `/Game/Gameplay/Crystal/BP_Crystall` OtherActor))
      (cast `BoxComponent` OtherComp)
      (set `self.AtWell` true))
    (:`then_2`
      ;;[1 1 1] Set AtChest
      (bind _asbp_chest (cast `/Game/Gameplay/Chest/BP_Chest` OtherActor))
      (cast `BoxComponent` OtherComp)
      (set `self.AtChest` true))
    (:`then_3`
      ;;[1 1 1] Set AtAnvil
      (bind _asbp_anvil (cast `/Game/Gameplay/Anvil/BP_Anvil` OtherActor))
      (cast `BoxComponent` OtherComp)
      (set `self.AtAnvil` true))))

(event `self.ReceiveBeginPlay`
  ;[1 1 1] BeginPlay
  (`/Engine/EditorBlueprintResources/StandardMacros.IsValid` (`self.PlayerUI`)
    (:`Is Valid`
      _)
    (:`Is Not Valid`
      (bind _returnvalue (`|CreateWidget` "/Game/UI/PlayerUI/UI_Player.UI_Player_C"))
      (bind _output_get (set `self.PlayerUI` _returnvalue))))
  (`UserWidget.AddToViewport` _output_get 0)
  (set `self.Health` 100.0)
  (set `self.Stamina` 100.0)
  (set `self.Mana` 100.0)
  (set `self.RessourcesRound` (`self.Ressources`)))

(event `InputAction|Interact`
  (params (Key :type "Key Structure"))
  (bind _collectedressources (`self.CollectedRessources`))
  ;[1 1 1] On Interact
  (:`Released`
    (if (== (`self.OpenUI`) null)
      (`|ExecutionSequence`
        (:`then_0`
          ;[1 1 1] Open UI_Well
          (`/Engine/EditorBlueprintResources/StandardMacros.IsValid` (stale `self.Capsule.OnComponentBeginOverlap` _asbp_crystall)
            (:`Is Valid`
              (if (and (or (`|GetArrayItem` _collectedressources) (`|GetArrayItem` _collectedressources 1)) (not (`/Game/Gameplay/Crystal/BP_Crystall.Active` (stale `self.Capsule.OnComponentBeginOverlap` _asbp_crystall))) (`self.AtWell`))
                (bind _uiref (`/Game/Gameplay/Crystal/BP_Crystall.OpenUI` (stale `self.Capsule.OnComponentBeginOverlap` _asbp_crystall)))
                (set `self.OpenUI` _uiref)
                (set `self.CanMove` false :!label _label)))))
        (:`then_1`
          ;[1 1 1] Open UI_Chest
          (`/Engine/EditorBlueprintResources/StandardMacros.IsValid` (stale `self.Capsule.OnComponentBeginOverlap` _asbp_chest)
            (:`Is Valid`
              (if (`self.AtChest`)
                (bind _uiref_2 (`/Game/Gameplay/Chest/BP_Chest.ToggelUI` (stale `self.Capsule.OnComponentBeginOverlap` _asbp_chest) true))
                (set `self.OpenUI` _uiref_2)
                (goto _label)))))
        (:`then_2`
          (`/Engine/EditorBlueprintResources/StandardMacros.IsValid` (stale `self.Capsule.OnComponentBeginOverlap` _asbp_anvil)
            (:`Is Valid`
              (if (`self.AtAnvil`)
                (bind _ui_ref (`/Game/Gameplay/Anvil/BP_Anvil.Toggel UI` (stale `self.Capsule.OnComponentBeginOverlap` _asbp_anvil) true))
                (set `self.OpenUI` _ui_ref)
                (goto _label))))))
      (else
        (`self.CloseOpenUI`)))))

(event `InputAction|Attack2`
  (params (Key :type "Key Structure"))
  ;[1 1 1] Inputs
  (:`Pressed`
    (if (not (`self.InBlacksmith`))
      (if (`|EnumEquality` (`self.PlayerAttack`) "NewEnumerator0")
        (bind _allow (`self.RemoveMana` 40.0))
        (if _allow
          (set `self.PlayerAttack` "NewEnumerator4")
          (`|ExecutionSequence`
            (:`then_0`
              (`self.Heal` (`self.HealAmount`)))
            (:`then_1`
              (set `self.IsAttacking` true :!label _label_2)))))))
  (:`Released`
    (set `self.IsAttacking` false :!label _label_3)))

(event `InputAction|Attack1`
  (params (Key :type "Key Structure"))
  ;[1 1 1] Inputs
  (:`Pressed`
    (if (not (`self.InBlacksmith`))
      (if (`|EnumEquality` (`self.PlayerAttack`) "NewEnumerator0")
        (bind _allow (`self.RemoveMana` 0.0))
        (if _allow
          (set `self.PlayerAttack` "NewEnumerator3")
          (goto _label_2)))))
  (:`Released`
    (goto _label_3)))

(event `self.ReceiveTick`
  (params (DeltaSeconds :type "Float (single-precision)"))
  ;[1 1 1] Camera Rotation and Player Movement
  (if (`self.CanMove`)
    (`self.Rotate` (`self.GetInputAxisValue`))
    (`self.Move` (`self.GetInputAxisValue`) (`self.GetInputAxisValue`))
    ;[1 1 1] StaminaReg
    (if (`self.StaminaRegOnCooldown`)
      (`KismetSystemLibrary.Delay` 1.5)
      (set `self.StaminaRegOnCooldown` false)
      (else
        (`self.AddStamina` (* DeltaSeconds 5.0))))))

(event `InputAction|Attack3`
  (params (Key :type "Key Structure"))
  ;[1 1 1] Inputs
  (:`Pressed`
    (if (not (`self.InBlacksmith`))
      (if (`|EnumEquality` (`self.PlayerAttack`) "NewEnumerator0")
        (bind _allow (`self.RemoveStamina` 10.0))
        (if _allow
          (set `self.PlayerAttack` "NewEnumerator1")
          (set `self.StaminaRegOnCooldown` true :!label _label_4)
          (goto _label_2)))))
  (:`Released`
    (goto _label_3)))

(event `InputAction|Attack4`
  (params (Key :type "Key Structure"))
  ;[1 1 1] Inputs
  (:`Pressed`
    (if (not (`self.InBlacksmith`))
      (if (`|EnumEquality` (`self.PlayerAttack`) "NewEnumerator0")
        (bind _allow (`self.RemoveStamina` 20.0))
        (if _allow
          (set `self.PlayerAttack` "NewEnumerator2")
          (goto _label_4)))))
  (:`Released`
    (goto _label_3)))

(event `OnRoundEnd`
  ;[1 1 1] OnRoundEnd
  (`self.AddRoundRessourcesToAll`)
  (set `self.Health` 100.0)
  (set `self.Stamina` 100.0))

(event `InputAction|Menu` :paused true
  (params (Key :type "Key Structure"))
  ;[1 1 1] Open / Close Pause Menu
  (:`Pressed`
    (if (`self.PauseMenuOpen`)
      (`self.ClosePauseMenu`)
      (else
        (`self.OpenPauseMenu`)))))

(event `self.ReceiveAnyDamage`
  (params (Damage :type "Float (single-precision)") (DamageType :type "DamageType Object Reference") (InstigatedBy :type "Controller Object Reference") (DamageCauser :type "Actor Object Reference"))
  ;[1 1 1] GetDamage
  (bind _output_get (set `self.Health` (- (`self.Health`) Damage)))
  (if (<= _output_get 0.0)
    (`self.Die`)))

(event `Die`
  ;[1 1 1] Die
  (`Widget.RemoveFromParent` (`self.PlayerUI`))
  (`KismetSystemLibrary.PrintString` "\"YouDie\""))

(fn `AddMana`
  (params (Amount :type "Float (double-precision)"))
  (bind _returnvalue (+ Amount (`self.Mana`)))
  (if (<= _returnvalue 100.0)
    (set `self.Mana` _returnvalue)
    (else
      (set `self.Mana` 100.0)))
  (return))

(fn `AddResource`
  (params (ResourceInput :type "Array of /Game/Gameplay/Resources/Ressources/BP_BaseResouces Object Reference"))
  (bind _ressources (`self.Ressources`))
  (for _array_element ResourceInput
    (bind _inventoryindex (`/Game/Gameplay/Resources/Ressources/BP_BaseResouces.InventoryIndex` _array_element))
    (bind _output (`|GetArrayItem` _ressources _inventoryindex))
    (bind _structout (setmembers `/Game/Gameplay/Resources/Struct_RessourceData` :`StructRef` _output :`Amount` (+ (`.Amount_13_95012F8242AB45B2BF5131860AD4EFD4` (break `/Game/Gameplay/Resources/Struct_RessourceData` _output)) 1)))
    (`KismetArrayLibrary.Array_Set` _ressources _inventoryindex _structout)
    (`self.K2_DestroyActor` _array_element)))

(fn `AddRessourcesRound`
  (params (Ressources :type "Array of /Game/Gameplay/Resources/Ressources/BP_BaseResouces Object Reference"))
  (bind _collectedressources (`self.CollectedRessources`))
  (bind _ressourcesround (`self.RessourcesRound`))
  (for _array_element Ressources
    (bind _inventoryindex (`/Game/Gameplay/Resources/Ressources/BP_BaseResouces.InventoryIndex` _array_element))
    (bind _output (`|GetArrayItem` _ressourcesround _inventoryindex))
    (bind _structout (setmembers `/Game/Gameplay/Resources/Struct_RessourceData` :`StructRef` _output :`Amount` (+ (`.Amount_13_95012F8242AB45B2BF5131860AD4EFD4` (break `/Game/Gameplay/Resources/Struct_RessourceData` _output)) 1)))
    (`KismetArrayLibrary.Array_Set` _ressourcesround _inventoryindex _structout)
    (if (not (`|GetArrayItem` _collectedressources _inventoryindex))
      (`KismetArrayLibrary.Array_Set` _collectedressources _inventoryindex true))
    (`self.K2_DestroyActor` _array_element)))

(fn `AddRoundRessourcesToAll`
  (bind _ressources (`self.Ressources`))
  (for (_array_element _array_index) (`self.RessourcesRound`)
    (bind _output (`|GetArrayItem` _ressources _array_index))
    (bind _structout (setmembers `/Game/Gameplay/Resources/Struct_RessourceData` :`StructRef` _output))
    (`KismetArrayLibrary.Array_Set` _ressources _array_index (make `/Game/Gameplay/Resources/Struct_RessourceData` (break `/Game/Gameplay/Resources/Struct_RessourceData` _structout) (+ (`.Amount_13_95012F8242AB45B2BF5131860AD4EFD4` (break `/Game/Gameplay/Resources/Struct_RessourceData` _output)) (`.Amount_13_95012F8242AB45B2BF5131860AD4EFD4` (break `/Game/Gameplay/Resources/Struct_RessourceData` _array_element))) (`.Rarity_10_CDDF21A8493A67EFA37913831D570883` (break `/Game/Gameplay/Resources/Struct_RessourceData` _structout)) (`.ItemDetails_7_5F49CCFC4B0C96AEE98292A5BE56A3EC` (break `/Game/Gameplay/Resources/Struct_RessourceData` _structout)) (`.Thumbnail_17_A746019B4F4F33B6CB39979F1D304AD2` (break `/Game/Gameplay/Resources/Struct_RessourceData` _structout)) (`.ArrayIndex_16_269F5AE34EFAB8B9B83769B13381073E` (break `/Game/Gameplay/Resources/Struct_RessourceData` _structout))))
    (bind _structout_2 (setmembers `/Game/Gameplay/Resources/Struct_RessourceData` :`StructRef` _array_element))
    (`KismetArrayLibrary.Array_Set` (`self.RessourcesRound`) _array_index (make `/Game/Gameplay/Resources/Struct_RessourceData` (break `/Game/Gameplay/Resources/Struct_RessourceData` _structout_2) 0 (`.Rarity_10_CDDF21A8493A67EFA37913831D570883` (break `/Game/Gameplay/Resources/Struct_RessourceData` _structout_2)) (`.ItemDetails_7_5F49CCFC4B0C96AEE98292A5BE56A3EC` (break `/Game/Gameplay/Resources/Struct_RessourceData` _structout_2)) (`.Thumbnail_17_A746019B4F4F33B6CB39979F1D304AD2` (break `/Game/Gameplay/Resources/Struct_RessourceData` _structout_2)) (`.ArrayIndex_16_269F5AE34EFAB8B9B83769B13381073E` (break `/Game/Gameplay/Resources/Struct_RessourceData` _structout_2)))))
  (return))

(fn `AddShieldRing`
  (params (UpgradedShield :type Boolean))
  (if UpgradedShield
    (bind _returnvalue (`AddComponent|NODE_AddInstancedStaticMeshComponent-7`))
    (`SceneComponent.K2_AttachToComponent` _returnvalue (`self.Shield`) "None" "SnapToTarget" "SnapToTarget" "SnapToTarget" true)))

(fn `AddStamina`
  (params (Amount :type "Float (double-precision)"))
  (bind _returnvalue (+ Amount (`self.Stamina`)))
  (if (<= _returnvalue 100.0)
    (set `self.Stamina` _returnvalue)
    (else
      (set `self.Stamina` 100.0)))
  (return))

(fn `AddWarAxeRing`
  (params (UpgradedWeapon :type Boolean))
  (if UpgradedWeapon
    (bind _returnvalue (`AddComponent|NODE_AddInstancedStaticMeshComponent-8`))
    (`SceneComponent.K2_AttachToComponent` _returnvalue (`self.Weapon`) "None" "SnapToTarget" "SnapToTarget" "SnapToTarget" true)))

(fn `AdjustHammerVisual`
  (params (HammerLevel :type Integer))
  (locals (HammerMeshesLv1 :type "Array of StaticMesh Object Reference") (HammerMeshesLv2 :type "Array of StaticMesh Object Reference") (HammerMeshesLv3 :type "Array of StaticMesh Object Reference") (HammerMeshesLv4 :type "Array of StaticMesh Object Reference") (HammerMeshesLv5 :type "Array of StaticMesh Object Reference") (HammerMeshesLv6 :type "Array of StaticMesh Object Reference") (HammerMeshesLv7 :type "Array of StaticMesh Object Reference") (HammerMeshesLv8 :type "Array of StaticMesh Object Reference") (HammerMeshesLv9 :type "Array of StaticMesh Object Reference") (HammerMeshesLv10 :type "Array of StaticMesh Object Reference") (HammerMeshesLv11 :type "Array of StaticMesh Object Reference") (HammerMeshesLv12 :type "Array of StaticMesh Object Reference") (HammerMeshesLv13 :type "Array of StaticMesh Object Reference") (HammerMeshesLv14 :type "Array of StaticMesh Object Reference") (HammerMeshesLv15 :type "Array of StaticMesh Object Reference") (HammerMeshesLv16 :type "Array of StaticMesh Object Reference") (HammerMeshesLv17 :type "Array of StaticMesh Object Reference") (HammerMeshesLv18 :type "Array of StaticMesh Object Reference"))
  (if (and (<= HammerLevel 35) (== (mod HammerLevel 2) 0))
    (bind _result (`/Engine/EditorBlueprintResources/StandardMacros.IncrementInt` (`self.VisualLevel`))
      (:`  `
        (switch `int` _result
          (:`2`
            (`self.SetHammerMeshes` (`local.HammerMeshesLv2`)))
          (:`3`
            (`self.SetHammerMeshes` (`local.HammerMeshesLv3`)))
          (:`4`
            (`self.SetHammerMeshes` (`local.HammerMeshesLv4`)))
          (:`5`
            (`self.SetHammerMeshes` (`local.HammerMeshesLv5`)))
          (:`6`
            (`self.SetHammerMeshes` (`local.HammerMeshesLv6`)))
          (:`7`
            (`self.SetHammerMeshes` (`local.HammerMeshesLv7`)))
          (:`8`
            (`self.SetHammerMeshes` (`local.HammerMeshesLv8`)))
          (:`9`
            (`self.SetHammerMeshes` (`local.HammerMeshesLv9`)))
          (:`10`
            (`self.SetHammerMeshes` (`local.HammerMeshesLv10`)))
          (:`11`
            (`self.SetHammerMeshes` (`local.HammerMeshesLv11`)))
          (:`12`
            (`self.SetHammerMeshes` (`local.HammerMeshesLv12`)))
          (:`13`
            (`self.SetHammerMeshes` (`local.HammerMeshesLv13`)))
          (:`14`
            (`self.SetHammerMeshes` (`local.HammerMeshesLv14`)))
          (:`15`
            (`self.SetHammerMeshes` (`local.HammerMeshesLv15`)))
          (:`16`
            (`self.SetHammerMeshes` (`local.HammerMeshesLv16`)))
          (:`17`
            (`self.SetHammerMeshes` (`local.HammerMeshesLv17`)))
          (:`18`
            (`self.SetHammerMeshes` (`local.HammerMeshesLv18`))))))))

(fn `CloseOpenUI`
  (bind _openui (`self.OpenUI`))
  (`|ExecutionSequence`
    (:`then_0`
      (bind _asui_well (cast `/Game/UI/CristalUI/UI_Well` _openui))
      (set `/Game/UI/CristalUI/UI_Well.PressedQuit` true _asui_well))
    (:`then_1`
      (bind _asui_chest (cast `/Game/UI/ChestUI/UI_Chest` _openui))
      (set `/Game/UI/ChestUI/UI_Chest.PressedQuit` true _asui_chest))
    (:`then_2`
      (bind _asui_anvil (cast `/Game/UI/AnvilUI/UI_Anvil` _openui))
      (set `/Game/UI/AnvilUI/UI_Anvil.PressedQuit` true _asui_anvil)))
  (set `self.OpenUI` null)
  (set `self.CanMove` true))

(fn `ClosePauseMenu`
  (bind _returnvalue (`GameplayStatics.GetPlayerController` 0))
  (bind _pausemenureference (`self.PauseMenuReference`))
  (`/Engine/EditorBlueprintResources/StandardMacros.IsValid` _pausemenureference
    (:`Is Valid`
      (`Widget.RemoveFromParent` _pausemenureference)
      (set `PlayerController.bShowMouseCursor` false _returnvalue)
      (`WidgetBlueprintLibrary.SetInputMode_GameOnly` _returnvalue)
      (`GameplayStatics.SetGamePaused` false)
      (set `self.PauseMenuOpen` false))))

(fn `Heal`
  (params (HealAmount :type "Float (double-precision)"))
  (bind _returnvalue (+ HealAmount (`self.Health`)))
  (if (> _returnvalue 100.0)
    (set `self.Health` 100.0)
    (else
      (set `self.Health` _returnvalue))))

(fn `LevelUpEnergyball`)

(fn `LevelUpHammer`
  (returns (`Sucsses?` :type Boolean))
  (if (>= (+ (`self.HammerLv`) 1) 37)
    (return false)
    (else
      (bind _result (`/Engine/EditorBlueprintResources/StandardMacros.IncrementInt` (`self.HammerLv`))
        (:`  `
          (`self.AdjustHammerVisual` _result)
          (`self.LevelUpPlayerLevel`)
          (return true))))))

(fn `LevelUpHeal`)

(fn `LevelUpHeavyAttack`)

(fn `LevelUpLightAttack`)

(fn `LevelUpPlayerLevel`)

(fn `OpenPauseMenu`
  (bind _returnvalue (`GameplayStatics.GetPlayerController` 0))
  (bind _pausemenureference (`self.PauseMenuReference`))
  (`/Engine/EditorBlueprintResources/StandardMacros.IsValid` (`self.PauseMenuReference`)
    (:`Is Valid`
      _)
    (:`Is Not Valid`
      (bind _returnvalue_2 (`|CreateWidget` "/Game/UI/PauseMenu/PauseMenu.PauseMenu_C"))
      (set `self.PauseMenuReference` _returnvalue_2)))
  (`WidgetBlueprintLibrary.SetInputMode_GameAndUIEx` _returnvalue _pausemenureference "DoNotLock" false)
  (set `PlayerController.bShowMouseCursor` true _returnvalue)
  (`UserWidget.AddToViewport` _pausemenureference 0)
  (`GameplayStatics.SetGamePaused` true)
  (set `self.PauseMenuOpen` true))

(fn `RemoveMana`
  (params (Amount :type "Float (double-precision)"))
  (returns (Allow :type Boolean))
  (bind _mana (`self.Mana`))
  (if (>= _mana Amount)
    (set `self.Mana` (- _mana Amount))
    (return true)
    (else
      (return false))))

(fn `RemoveResource`
  (params (Resource :type "Array of /Game/Gameplay/Resources/Ressources/BP_BaseResouces Object Reference"))
  (bind _ressources (`self.Ressources`))
  (for _array_element Resource
    (bind _inventoryindex (`/Game/Gameplay/Resources/Ressources/BP_BaseResouces.InventoryIndex` _array_element))
    (bind _output (`|GetArrayItem` _ressources _inventoryindex))
    (bind _returnvalue (+ (`.Amount_13_95012F8242AB45B2BF5131860AD4EFD4` (break `/Game/Gameplay/Resources/Struct_RessourceData` _output)) -1))
    (if (<= _returnvalue 0)
      (`KismetSystemLibrary.PrintString` "You dont have the needed Resources")
      (else
        (bind _structout (setmembers `/Game/Gameplay/Resources/Struct_RessourceData` :`StructRef` _output :`Amount` _returnvalue))
        (`KismetArrayLibrary.Array_Set` _ressources _inventoryindex _structout)))))

(fn `RemoveRessourceByIndex`
  (params (Inde :type Integer) (Amount :type Integer))
  (returns (Sucsse :type Boolean))
  (bind _ressources (`self.Ressources`))
  (bind (_output_itemname _output_amount _output_rarity _output_itemdetails _output_thumbnail _output_arrayindex) (break `/Game/Gameplay/Resources/Struct_RessourceData` (`|GetArrayItem` _ressources Inde)))
  (if (>= _output_amount Amount)
    (`KismetArrayLibrary.Array_Set` _ressources _output_arrayindex (make `/Game/Gameplay/Resources/Struct_RessourceData` _output_itemname (- _output_amount Amount) _output_rarity _output_itemdetails _output_thumbnail _output_arrayindex))
    (return true)
    (else
      (return false))))

(fn `RemoveStamina`
  (params (Amount :type "Float (double-precision)"))
  (returns (Allow :type Boolean))
  (bind _stamina (`self.Stamina`))
  (if (>= _stamina Amount)
    (set `self.Stamina` (- _stamina Amount))
    (return true)
    (else
      (return false))))

(fn `SetHammerMeshes`
  (params (Meshes :type "Array of StaticMesh Object Reference"))
  (`|ExecutionSequence`
    (:`then_0`
      (`StaticMeshComponent.SetStaticMesh` (`self.WeaponHead1`) (`|GetArrayItem` Meshes)))
    (:`then_1`
      (`StaticMeshComponent.SetStaticMesh` (`self.WeaponHead2`) (`|GetArrayItem` Meshes 1)))
    (:`then_2`
      (`StaticMeshComponent.SetStaticMesh` (`self.WeaponHead3`) (`|GetArrayItem` Meshes 2)))
    (:`then_3`
      (`StaticMeshComponent.SetStaticMesh` (`self.WeaponHandle`) (`|GetArrayItem` Meshes 3)))
    (:`then_4`
      (`StaticMeshComponent.SetStaticMesh` (`self.WeaponEnd`) (`|GetArrayItem` Meshes 4)))
    (:`then_5`
      (`StaticMeshComponent.SetStaticMesh` (`self.WeaponTip`) (`|GetArrayItem` Meshes 5)))
    (:`then_6`
      (`StaticMeshComponent.SetStaticMesh` (`self.WeaponMounting`) (`|GetArrayItem` Meshes 6)))))

(fn `SpawnEnergyball`
  (bind _returnvalue (`|SpawnActorFromClass` "/Game/Characters/PC/Blueprints/BP_Energyball.BP_Energyball_C" (`self.GetTransform`) "AlwaysSpawn" "OverrideRootScale" null null))
  (`/Engine/EditorBlueprintResources/StandardMacros.IsValid` _returnvalue
    (:`Is Valid`
      (`ProjectileMovementComponent.SetVelocityInLocalSpace` (`/Game/Characters/PC/Blueprints/BP_Energyball.ProjectileMovement` _returnvalue) (* (`SceneComponent.GetForwardVector` (`self.Mesh`)) -2000)))))

(fn `UserConstructionScript`)