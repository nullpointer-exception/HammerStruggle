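; Player character Blueprint handling movement, attack input, resource pickup, health and the pause menu.
; Tick feeds axis values into Rotate and Move, while Attack3 holds IsAttacking true and collector overlaps store resources and destroy their actors.
; Damage lowers Health until Die, which only prints a message.
; The pause menu widget is created once and reused, and helper functions attach instanced-mesh upgrade rings to Shield and Weapon.
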(event `self.ReceiveTick`
  (params (DeltaSeconds :type "Float (single-precision)"))
  ;[1 1 1] Camera Rotation and Player Movement
  (`self.Rotate` (`self.GetInputAxisValue`))
  (`self.Move` (`self.GetInputAxisValue`) (`self.GetInputAxisValue`)))

(event `InputAction|Menu` :paused true
  (params (Key :type "Key Structure"))
  ;[1 1 1] Open Pause Menu
  (:`Pressed`
    (if (`self.PauseMenuOpen`)
      (`self.ClosePauseMenu`)
      (else
        (`self.OpenPauseMenu`)))))

(event `InputAction|Attack3`
  (params (Key :type "Key Structure"))
  (:`Pressed`
    (set `self.IsAttacking` true))
  (:`Released`
    (set `self.IsAttacking` false)))

(event `self.ResouceCollector.OnComponentBeginOverlap`
  (params (OverlappedComponent :type "PrimitiveComponent Object Reference") (OtherActor :type "Actor Object Reference") (OtherComp :type "PrimitiveComponent Object Reference") (OtherBodyIndex :type Integer) (bFromSweep :type Boolean) (SweepResult :type "HitResult Structure (by ref)"))
  (bind _asbp_base_resouces (cast `/Game/Gameplay/Resources/BP_BaseResouces` OtherActor))
  (`self.AddResource` _asbp_base_resouces)
  (`self.K2_DestroyActor` _asbp_base_resouces)
  ;[1 1 1] Log Print
  (for _array_element (`self.Resources`)
    (`KismetSystemLibrary.PrintString` (`KismetSystemLibrary.GetDisplayName` _array_element)))
  (`KismetSystemLibrary.PrintString` "Inventory:"))

(event `self.ReceiveAnyDamage`
  (params (Damage :type "Float (single-precision)") (DamageType :type "DamageType Object Reference") (InstigatedBy :type "Controller Object Reference") (DamageCauser :type "Actor Object Reference"))
  (bind _health (`self.Health`))
  (bind _output_get (set `self.Health` (- _health Damage)))
  (`KismetSystemLibrary.PrintString` (`KismetStringLibrary.Conv_DoubleToString` _health))
  (if (<= _output_get 0.0)
    (`self.Die`)))

(event `Die`
  (`KismetSystemLibrary.PrintString` "\"YouDie\""))

(fn `AddResource`
  (params (Resource :type "/Game/Gameplay/Resources/BP_BaseResouces Object Reference"))
  (`KismetArrayLibrary.Array_Add` (`self.Resources`) Resource))

(fn `AddShieldRing`
  (params (UpgradedShield :type Boolean))
  (if UpgradedShield
    (bind _returnvalue (`AddComponent|NODE_AddInstancedStaticMeshComponent-7`))
    (`SceneComponent.K2_AttachToComponent` _returnvalue (`self.Shield`) "None" "SnapToTarget" "SnapToTarget" "SnapToTarget" true)))

(fn `AddWarAxeRing`
  (params (UpgradedWeapon :type Boolean))
  (if UpgradedWeapon
    (bind _returnvalue (`AddComponent|NODE_AddInstancedStaticMeshComponent-8`))
    (`SceneComponent.K2_AttachToComponent` _returnvalue (`self.Weapon`) "None" "SnapToTarget" "SnapToTarget" "SnapToTarget" true)))

(fn `ClosePauseMenu`
  (bind _returnvalue (`GameplayStatics.GetPlayerController` 0))
  (bind _pausemenureference (`self.PauseMenuReference`))
  (`/Engine/EditorBlueprintResources/StandardMacros.IsValid` _pausemenureference
    (:`Is Valid`
      (`Widget.RemoveFromParent` _pausemenureference)
      (set `PlayerController.bShowMouseCursor` false _returnvalue)
      (`WidgetBlueprintLibrary.SetInputMode_GameOnly` _returnvalue)
      (`GameplayStatics.SetGamePaused` false)
      (set `self.PauseMenuOpen` false))))

(fn `OpenPauseMenu`
  (bind _returnvalue (`GameplayStatics.GetPlayerController` 0))
  (bind _pausemenureference (`self.PauseMenuReference`))
  (`/Engine/EditorBlueprintResources/StandardMacros.IsValid` (`self.PauseMenuReference`)
    (:`Is Valid`
      _)
    (:`Is Not Valid`
      (bind _returnvalue_2 (`|CreateWidget` "/Game/UI/PauseMenu/PauseMenu.PauseMenu_C"))
      (set `self.PauseMenuReference` _returnvalue_2)))
  (`WidgetBlueprintLibrary.SetInputMode_GameAndUIEx` _returnvalue _pausemenureference "DoNotLock" false)
  (set `PlayerController.bShowMouseCursor` true _returnvalue)
  (`UserWidget.AddToViewport` _pausemenureference 0)
  (`GameplayStatics.SetGamePaused` true)
  (set `self.PauseMenuOpen` true))

(fn `RemoveResource`
  (params (Resource :type "/Game/Gameplay/Resources/BP_BaseResouces Object Reference"))
  (`KismetArrayLibrary.Array_RemoveItem` (`self.Resources`) Resource))

(fn `UserConstructionScript`)