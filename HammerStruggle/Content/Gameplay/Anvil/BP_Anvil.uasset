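; Anvil Blueprint that opens and closes the UI_Anvil upgrade widget and calculates hammer and LA upgrade costs.
; ToggelUI reuses one widget and switches input mode and cursor, while Tick polls its PressedQuit flag to close it.
; Next-level costs fill array slots, zeroed when not positive: four quadratic curves for hammer, logarithmic curves for LA.
; LA's first slot never receives its computed cost, and its fourth slot and return are unreachable.
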(event `self.ReceiveTick`
  (params (DeltaSeconds :type "Float (single-precision)"))
  (bind _uiref (`self.UIRef`))
  (`/Engine/EditorBlueprintResources/StandardMacros.IsValid` _uiref
    (:`Is Valid`
      (if (`/Game/UI/AnvilUI/UI_Anvil.PressedQuit` _uiref)
        (`self.Toggel UI` false)))))

(fn `CalculateCostHammer`
  (params (Level :type Integer) (A :type "Float (double-precision)") (B :type "Float (double-precision)") (C :type "Float (double-precision)"))
  (returns (IsOverZero :type Boolean) (Cost :type Integer))
  (bind _returnvalue (`KismetMathLibrary.Conv_IntToDouble` Level))
  (bind _returnvalue_2 (+ (+ (* (`KismetMathLibrary.Square` _returnvalue) A) (* _returnvalue B)) C))
  (if (> _returnvalue_2 0.0)
    (return true (`KismetMathLibrary.Round` _returnvalue_2))
    (else
      (return false 0))))

(fn `CalculateCostUpgrades`
  (params (CurrLevel :type Integer) (A :type "Float (double-precision)") (C :type "Float (double-precision)"))
  (returns (IsOverZero :type Boolean) (Cost :type Integer))
  (bind _returnvalue (`KismetMathLibrary.Round` (+ (* (`KismetMathLibrary.Loge` (`KismetMathLibrary.Conv_IntToDouble` CurrLevel)) A) C)))
  (if (> _returnvalue 0)
    (return true _returnvalue)
    (else
      (return false 0))))

(fn `SetCostHammerUpgrade`
  (params (CurrLevel :type Integer))
  (returns (NextLevel :type Integer) (Cost :type "Array of Integer"))
  (locals (Output :type "Array of Integer"))
  (bind _returnvalue (+ CurrLevel 1))
  (bind _output (`local.Output`))
  (`|ExecutionSequence`
    (:`then_0`
      ;[1 1 1] Set if Over Zero
      (bind (_isoverzero _cost) (`self.CalculateCostHammer` _returnvalue -0.2631 5.2631))
      (if _isoverzero
        (`KismetArrayLibrary.Array_Set` _output 0 _cost)
        (else
          ;[1 1 1] Set to Zero to not break the Sequenz
          (`KismetArrayLibrary.Array_Set` _output))))
    (:`then_1`
      (bind (_isoverzero_2 _cost_2) (`self.CalculateCostHammer` _returnvalue -0.2631 10.5263 -78.947304))
      (if _isoverzero_2
        (`KismetArrayLibrary.Array_Set` _output 1 _cost_2)
        (else
          (`KismetArrayLibrary.Array_Set` _output 1))))
    (:`then_2`
      (bind (_isoverzero_3 _cost_3) (`self.CalculateCostHammer` _returnvalue -0.2631 15.7894 -210.526001))
      (if _isoverzero_3
        (`KismetArrayLibrary.Array_Set` _output 2 _cost_3)
        (else
          (`KismetArrayLibrary.Array_Set` _output 2))))
    (:`then_3`
      (bind (_isoverzero_4 _cost_4) (`self.CalculateCostHammer` _returnvalue -0.2631 24.7619 -464.285706))
      (if _isoverzero_4
        (`KismetArrayLibrary.Array_Set` _output 3 _cost_4)
        (else
          (`KismetArrayLibrary.Array_Set` _output 3)))
      (return _returnvalue _output))))

(fn `SetCostLA_Upgrade`
  (params (CurrLevel :type Integer))
  (returns (NextLevel :type Integer) (Cost :type "Array of Integer"))
  (locals (Output :type "Array of Integer"))
  (bind _returnvalue (+ CurrLevel 1))
  (bind _output (`local.Output`))
  (`|ExecutionSequence`
    (:`then_0`
      ;[1 1 1] Set if Over Zero
      (bind _isoverzero (`self.CalculateCostUpgrades` _returnvalue 1.4 4.0))
      (if _isoverzero
        (`KismetArrayLibrary.Array_Set` _output)
        (else
          (`KismetArrayLibrary.Array_Set` _output))))
    (:`then_1`
      (bind (_isoverzero_2 _cost) (`self.CalculateCostUpgrades` _returnvalue 1.8 4.0))
      (if _isoverzero_2
        (`KismetArrayLibrary.Array_Set` _output 1 _cost)
        (else
          (`KismetArrayLibrary.Array_Set` _output 1))))
    (:`then_2`
      (bind (_isoverzero_3 _cost_2) (`self.CalculateCostUpgrades` _returnvalue 2.2 4.0))
      (if _isoverzero_3
        (`KismetArrayLibrary.Array_Set` _output 2 _cost_2)
        (else
          (`KismetArrayLibrary.Array_Set` _output 2))))))

(fn `Toggel UI`
  (params (`Open?` :type Boolean))
  (returns (`UI Ref` :type "/Game/UI/AnvilUI/UI_Anvil Object Reference"))
  (bind _returnvalue (`GameplayStatics.GetPlayerController` 0))
  (bind _uiref (`self.UIRef`))
  (bind _uiref_2 (`self.UIRef`))
  (if `Open?`
    (`/Engine/EditorBlueprintResources/StandardMacros.IsValid` _uiref
      (:`Is Valid`
        _)
      (:`Is Not Valid`
        (bind _returnvalue_2 (`|CreateWidget` "/Game/UI/AnvilUI/UI_Anvil.UI_Anvil_C"))
        (set `self.UIRef` _returnvalue_2)
        (set `/Game/UI/AnvilUI/UI_Anvil.AnvilRef` self _uiref_2)))
    (`WidgetBlueprintLibrary.SetInputMode_GameAndUIEx` _returnvalue _uiref_2 "DoNotLock" false)
    (set `PlayerController.bShowMouseCursor` true _returnvalue)
    (`UserWidget.AddToViewport` _uiref_2 0)
    (return _uiref_2)
    (else
      (`/Engine/EditorBlueprintResources/StandardMacros.IsValid` _uiref
        (:`Is Valid`
          (`Widget.RemoveFromParent` _uiref)
          (set `PlayerController.bShowMouseCursor` false _returnvalue)
          (`WidgetBlueprintLibrary.SetInputMode_GameOnly` _returnvalue)
          (set `/Game/UI/AnvilUI/UI_Anvil.PressedQuit` false _uiref)
          (return null))))))

(fn `UserConstructionScript`)