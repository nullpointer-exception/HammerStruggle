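; Enemy spawner for wave rounds that spawns melee and throwing golems on a delay, each assigned a resource.
; Golem count, damage and health scale with the round controller's WaveStrength.
; A resource pool starts as wood or stone, then RoundCount thresholds overwrite entries with rarer tiers using quadratic chances, and recursive random picks draw from it.
; Living golems are tracked in LeftGolems; removing the last triggers the controller's Collecting phase.
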(event `StartSpawn`
  (set `self.MaxGolemAmount` (+ (`/Game/Gameplay/Round/BP_RoundController.WaveStrength` (`self.RoundControllerRef`)) 1))
  (`self.Calculate_GolemDamage`)
  (`self.Calculate_GolemHealth`)
  (`self.Callculate Ressources`)
  (`self.ForLoop Delay` 0 (- (`self.MaxGolemAmount`) 1) 1.5
    (:`Loop Body`
      (`self.SpawnEnemy`))))

(fn `Calculate_GolemDamage`
  (locals (Slope :type "Float (double-precision)" :default 1.0) (BaseDamage :type "Float (double-precision)" :default 10.0))
  (set `self.GolemDamage` (+ (`local.BaseDamage`) (* (`/Game/Gameplay/Round/BP_RoundController.WaveStrength` (`self.RoundControllerRef`)) (`local.Slope`)))))

(fn `Calculate_GolemHealth`
  (locals (Slope :type "Float (double-precision)" :default 1.6) (BaseHealth :type "Float (double-precision)" :default 100.0))
  (set `self.GolemHealth` (`KismetMathLibrary.Round` (+ (`local.BaseHealth`) (* (`/Game/Gameplay/Round/BP_RoundController.WaveStrength` (`self.RoundControllerRef`)) (`local.Slope`))))))

(fn `Callculate Ressources`
  (bind _roundcount (`/Game/Gameplay/Round/BP_RoundController.RoundCount` (`self.RoundControllerRef`)))
  (`KismetArrayLibrary.Array_Clear` (`self.Ressources`))
  (`KismetArrayLibrary.Array_Clear` (`self.UsedIndex`))
  (`|ExecutionSequence`
    (:`then_0`
      ;[1 1 1] Under Wave 10
      (for _index (range (`self.MaxGolemAmount`))
        (switch `int` (`KismetMathLibrary.RandomInteger` 2)
          (:`0`
            (`KismetArrayLibrary.Array_Set` (`self.Ressources`) _index "/Game/Gameplay/Resources/Ressources/BP_Ressource_Wood.BP_Ressource_Wood_C" true))
          (:`1`
            (`KismetArrayLibrary.Array_Set` (`self.Ressources`) _index "/Game/Gameplay/Resources/Ressources/BP_Ressource_Stone.BP_Ressource_Stone_C" true)))))
    (:`then_1`
      (if (>= _roundcount 10)
        ;[1 1 1] <10 | >25
        ;;[0.5245 0.7717 1] Rare
        (switch `int` (`KismetMathLibrary.RandomInteger` 2)
          (:`0`
            (`KismetArrayLibrary.Array_Set` (`self.Ressources`) 0 "/Game/Gameplay/Resources/Ressources/BP_Ressource_Copper.BP_Ressource_Copper_C"))
          (:`1`
            (`KismetArrayLibrary.Array_Set` (`self.Ressources`) 0 "/Game/Gameplay/Resources/Ressources/BP_Ressource_Iron.BP_Ressource_Iron_C")))
        (bind _probability (`self.GetProbabilityRare` (`/Game/Gameplay/Round/BP_RoundController.RoundCount` (`self.RoundControllerRef`))))
        (for _index_2 (range 1 (`self.MaxGolemAmount`))
          (if (<= (`KismetMathLibrary.RandomFloatInRange` 0.0 100.0) _probability)
            (switch `int` (`KismetMathLibrary.RandomInteger` 2)
              (:`0`
                (`KismetArrayLibrary.Array_Set` (`self.Ressources`) _index_2 "/Game/Gameplay/Resources/Ressources/BP_Ressource_Iron.BP_Ressource_Iron_C"))
              (:`1`
                (`KismetArrayLibrary.Array_Set` (`self.Ressources`) _index_2 "/Game/Gameplay/Resources/Ressources/BP_Ressource_Copper.BP_Ressource_Copper_C")))))))
    (:`then_2`
      (if (>= _roundcount 25)
        ;[1 1 1] <25 | >50
        ;;[0.972 0.5109 1] Epic
        (switch `int` (`KismetMathLibrary.RandomInteger` 2)
          (:`0`
            (`KismetArrayLibrary.Array_Set` (`self.Ressources`) 0 "/Game/Gameplay/Resources/Ressources/BP_Ressource_Marbel.BP_Ressource_Marbel_C"))
          (:`1`
            (`KismetArrayLibrary.Array_Set` (`self.Ressources`) 0 "/Game/Gameplay/Resources/Ressources/BP_Ressource_Silver.BP_Ressource_Silver_C")))
        (bind _probability_2 (`self.GetProbabilityEpic` (`/Game/Gameplay/Round/BP_RoundController.RoundCount` (`self.RoundControllerRef`))))
        (for _index_3 (range 1 (`self.MaxGolemAmount`))
          (if (<= (`KismetMathLibrary.RandomFloatInRange` 0.0 100.0) _probability_2)
            (switch `int` (`KismetMathLibrary.RandomInteger` 2)
              (:`0`
                (`KismetArrayLibrary.Array_Set` (`self.Ressources`) _index_3 "/Game/Gameplay/Resources/Ressources/BP_Ressource_Marbel.BP_Ressource_Marbel_C"))
              (:`1`
                (`KismetArrayLibrary.Array_Set` (`self.Ressources`) _index_3 "/Game/Gameplay/Resources/Ressources/BP_Ressource_Silver.BP_Ressource_Silver_C")))))))
    (:`then_3`
      (if (>= _roundcount 50)
        ;[1 1 1] Over 50
        ;;[1 0.8826 0.3051] Legendery
        (switch `int` (`KismetMathLibrary.RandomInteger` 2)
          (:`0`
            (`KismetArrayLibrary.Array_Set` (`self.Ressources`) 0 "/Game/Gameplay/Resources/Ressources/BP_Ressource_Gem.BP_Ressource_Gem_C"))
          (:`1`
            (`KismetArrayLibrary.Array_Set` (`self.Ressources`) 0 "/Game/Gameplay/Resources/Ressources/BP_Ressource_Gold.BP_Ressource_Gold_C")))
        (bind _probability_3 (`self.GetProbabilityRare` (`/Game/Gameplay/Round/BP_RoundController.RoundCount` (`self.RoundControllerRef`))))
        (for _index_4 (range 1 (`self.MaxGolemAmount`))
          (if (<= (`KismetMathLibrary.RandomFloatInRange` 0.0 100.0) _probability_3)
            (switch `int` (`KismetMathLibrary.RandomInteger` 2)
              (:`0`
                (`KismetArrayLibrary.Array_Set` (`self.Ressources`) _index_4 "/Game/Gameplay/Resources/Ressources/BP_Ressource_Marbel.BP_Ressource_Marbel_C"))
              (:`1`
                (`KismetArrayLibrary.Array_Set` (`self.Ressources`) _index_4 "/Game/Gameplay/Resources/Ressources/BP_Ressource_Silver.BP_Ressource_Silver_C")))))))))

(fn `Get Random Ressource Test`
  (returns (Ressouce :type "/Game/Gameplay/Resources/Ressources/BP_BaseResouces Class Reference"))
  (locals (Output :type "/Game/Gameplay/Resources/Ressources/BP_BaseResouces Class Reference"))
  (bind _ressources (`self.Ressources`))
  (bind _output (`|GetArrayItem` _ressources (`KismetMathLibrary.RandomIntegerInRange` 0 (- (`KismetArrayLibrary.Array_Length` _ressources) 1))))
  (for (_array_element _array_index) _ressources
    (`KismetSystemLibrary.PrintString` (`KismetStringLibrary.Concat_StrStr` (`KismetStringLibrary.Conv_IntToString` _array_index) " | " (`KismetSystemLibrary.GetClassDisplayName` _array_element)) true true (struct :`G` 0.66 :`B` 1.0 :`A` 1.0) 15.0))
  (`KismetSystemLibrary.PrintString` "----------------------" true true (struct :`G` 0.66 :`B` 1.0 :`A` 1.0) 15.0)
  (bind _output_get (set `local.Output` _output))
  (`KismetSystemLibrary.PrintString` (`KismetStringLibrary.Concat_StrStr` "Output: " (`KismetSystemLibrary.GetClassDisplayName` _output_get)) true true (struct :`G` 0.66 :`B` 1.0 :`A` 1.0) 15.0)
  (bind _returnvalue (`KismetArrayLibrary.Array_RemoveItem` _ressources _output))
  (if _returnvalue
    (return (`local.Output`))))

(fn `GetProbabilityEpic`
  (params (RoundCount :type Integer))
  (returns (Probability :type "Float (double-precision)"))
  (locals (a :type "Float (double-precision)" :default 0.08) (b :type "Float (double-precision)" :default 2.0))
  (bind _returnvalue (`KismetMathLibrary.Conv_IntToDouble` RoundCount))
  (return (- (* (`local.a`) (`KismetMathLibrary.Square` _returnvalue)) (* (`local.b`) _returnvalue))))

(fn `GetProbabilityLegendery`
  (params (RoundCount :type Integer))
  (returns (Probability :type "Float (double-precision)"))
  (locals (a :type "Float (double-precision)" :default 0.02) (b :type "Float (double-precision)" :default 1.0))
  (bind _returnvalue (`KismetMathLibrary.Conv_IntToDouble` RoundCount))
  (return (- (* (`local.a`) (`KismetMathLibrary.Square` _returnvalue)) (* (`local.b`) _returnvalue))))

(fn `GetProbabilityRare`
  (params (RoundCount :type Integer))
  (returns (Probability :type "Float (double-precision)"))
  (locals (a :type "Float (double-precision)" :default 0.267) (b :type "Float (double-precision)" :default 2.667))
  (bind _returnvalue (`KismetMathLibrary.Conv_IntToDouble` RoundCount))
  (return (- (* (`local.a`) (`KismetMathLibrary.Square` _returnvalue)) (* (`local.b`) _returnvalue))))

(fn `GetRandomRessource`
  (returns (Ressouce :type "/Game/Gameplay/Resources/Ressources/BP_BaseResouces Class Reference"))
  (locals (Output :type "/Game/Gameplay/Resources/Ressources/BP_BaseResouces Class Reference"))
  (bind _ressources (`self.Ressources`))
  (bind _usedindex (`self.UsedIndex`))
  (bind _returnvalue (`KismetMathLibrary.RandomIntegerInRange` 0 (- (`KismetArrayLibrary.Array_Length` _ressources) 1)))
  (if (`KismetArrayLibrary.Array_Contains` _usedindex _returnvalue)
    (bind _ressouce (`self.GetRandomRessource`))
    (return _ressouce)
    (else
      (set `local.Output` (`|GetArrayItem` _ressources _returnvalue))
      (`KismetArrayLibrary.Array_Add` _usedindex _returnvalue)
      (return (`local.Output`)))))

(fn `RemoveFromList`
  (params (GolemToRemove :type "/Game/Characters/NPC/Enemies/KI/BP_AIBase Object Reference"))
  (bind _leftgolems (`self.LeftGolems`))
  (if (`KismetArrayLibrary.Array_Contains` _leftgolems GolemToRemove)
    (`KismetArrayLibrary.Array_RemoveItem` _leftgolems GolemToRemove)
    (if (<= (`KismetArrayLibrary.Array_Length` _leftgolems) 0)
      (`/Game/Gameplay/Round/BP_RoundController.Collecting` (`self.RoundControllerRef`)))))

(fn `SpawnEnemy`
  (bind (_newparam_location _newparam_rotation) (`KismetMathLibrary.BreakTransform` (`self.SpawnPoint`)))
  (bind (_newparam_location_2 _newparam_rotation_2) (`KismetMathLibrary.BreakTransform` (`self.SpawnPoint`)))
  (bind _leftgolems (`self.LeftGolems`))
  (bind _golemdamage (`self.GolemDamage`))
  (bind _returnvalue (`KismetMathLibrary.Conv_IntToDouble` (`self.GolemHealth`)))
  (switch `int` (`KismetMathLibrary.RandomIntegerInRange` 0 1)
    (:`0`
      ;[1 1 1] Throw
      (bind _returnvalue_2 (`AIBlueprintHelperLibrary.SpawnAIFromClass` "/Game/Characters/NPC/Enemies/KI/Throw/Blueprints/BP_AI_Throw_CharacterFix.BP_AI_Throw_CharacterFix_C" "/Game/Characters/NPC/Enemies/KI/Throw/BB_BT/BT_Throw.BT_Throw" _newparam_location_2 _newparam_rotation_2))
      (bind _asbp_aibase (cast `/Game/Characters/NPC/Enemies/KI/BP_AIBase` _returnvalue_2))
      (`KismetArrayLibrary.Array_AddUnique` _leftgolems _asbp_aibase)
      (bind _ressouce (`self.GetRandomRessource`))
      (`/Game/Characters/NPC/Enemies/KI/BP_AIBase.SetRessource` _asbp_aibase _ressouce)
      (set `/Game/Characters/NPC/Enemies/KI/BP_AIBase.EnemySpawnerRef` self _asbp_aibase)
      (set `/Game/Characters/NPC/Enemies/KI/BP_AIBase.DamageMeele` _golemdamage _asbp_aibase)
      (set `/Game/Characters/NPC/Enemies/KI/BP_AIBase.DamageThrow` _golemdamage _asbp_aibase)
      (set `/Game/Characters/NPC/Enemies/KI/BP_AIBase.Health` _returnvalue _asbp_aibase))
    (:`1`
      ;[1 1 1] Meele
      (bind _returnvalue_3 (`AIBlueprintHelperLibrary.SpawnAIFromClass` "/Game/Characters/NPC/Enemies/KI/Melee/Blueprints/BP_AI_Melee_Character.BP_AI_Melee_Character_C" "/Game/Characters/NPC/Enemies/KI/Melee/BB_BT/BT_Melee.BT_Melee" _newparam_location _newparam_rotation))
      (bind _asbp_aibase_2 (cast `/Game/Characters/NPC/Enemies/KI/BP_AIBase` _returnvalue_3))
      (`KismetArrayLibrary.Array_AddUnique` _leftgolems _asbp_aibase_2)
      (bind _ressouce_2 (`self.GetRandomRessource`))
      (`/Game/Characters/NPC/Enemies/KI/BP_AIBase.SetRessource` _asbp_aibase_2 _ressouce_2)
      (set `/Game/Characters/NPC/Enemies/KI/BP_AIBase.EnemySpawnerRef` self _asbp_aibase_2)
      (set `/Game/Characters/NPC/Enemies/KI/BP_AIBase.DamageMeele` _golemdamage _asbp_aibase_2)
      (set `/Game/Characters/NPC/Enemies/KI/BP_AIBase.Health` _returnvalue _asbp_aibase_2))))

(fn `UserConstructionScript`)