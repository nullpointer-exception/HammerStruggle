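; BP_RoundController runs the game's round loop, tracking round status and count for the player found at BeginPlay.
; StartRound computes wave strength from round count and player level, then, if the player is outside the blacksmith, toggles its doors, increments the count and starts the enemy spawner.
; Collecting toggles the doors back to their initial state, and EndRound resets the status to its starting value.
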(event `self.ReceiveBeginPlay`
  (bind _asbp_hsplayer (cast `/Game/Characters/Player/Blueprints/BP_HSPlayer` (`GameplayStatics.GetPlayerPawn` 0))
    (:`then`
      (set `self.PlayerRef` _asbp_hsplayer)
      (set `self.RoundStatus` "NewEnumerator1")
      (`self.BeginGame`))
    (:`CastFailed`
      (`KismetSystemLibrary.PrintString` "No Player found"))))

(fn `BeginGame`
  (`/Game/Environment/Buildings/BP_HSBlacksmith.ToggelDoors` (`self.BlacksmithRef`) true))

(fn `Calculate_WaveStrength`
  (set `self.WaveStrength` (`KismetMathLibrary.FCeil` (* (+ (`KismetMathLibrary.FTrunc` (* (`self.RoundCount`) 0.5)) (`/Game/Characters/Player/Blueprints/BP_HSPlayer.PlayerLevel` (`self.PlayerRef`))) 0.5))))

(fn `Collecting`
  (set `self.RoundStatus` "NewEnumerator3")
  (`/Game/Environment/Buildings/BP_HSBlacksmith.ToggelDoors` (`self.BlacksmithRef`) true))

(fn `EndRound`
  (set `self.RoundStatus` "NewEnumerator1"))

(fn `StartRound`
  (`self.Calculate_WaveStrength`)
  (if (not (`/Game/Environment/Buildings/BP_HSBlacksmith.IsPlayerInside` (`self.BlacksmithRef`)))
    (set `self.RoundStatus` "NewEnumerator2")
    (`/Game/Environment/Buildings/BP_HSBlacksmith.ToggelDoors` (`self.BlacksmithRef`) false)
    (bind _result (`/Engine/EditorBlueprintResources/StandardMacros.IncrementInt` (`self.RoundCount`))
      (:`  `
        (set `self.RoundCount` _result)
        (`/Game/Gameplay/Round/BP_EnemySpawner.StartSpawn` (`self.EnemySpawnerRef`))))))

(fn `UserConstructionScript`)