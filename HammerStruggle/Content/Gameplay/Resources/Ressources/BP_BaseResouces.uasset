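; Base resource pickup Blueprint that hovers, spins and can fly toward the player.
; The construction script caches the spawn position, and Tick moves the Scene component around it with a sine-driven vertical lerp plus yaw rotation.
; While IsCollectable is set, Tick also issues a short MoveComponentTo toward the BP_HSPlayer capsule, alongside the still-running hover update.
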(event `self.ReceiveTick`
  (params (DeltaSeconds :type "Float (single-precision)"))
  (bind (_spawnpos_x _spawnpos_y _spawnpos_z) (`KismetMathLibrary.BreakVector` (`self.SpawnPos`)))
  (bind _offsetz (`self.OffsetZ`))
  (bind _scene (`self.Scene`))
  (`|ExecutionSequence`
    (:`then_0`
      ;[1 1 1] Fly To Player
      (if (`self.IsCollectable`)
        (bind _asbp_hsplayer (cast `/Game/Characters/Player/Blueprints/BP_HSPlayer` (`GameplayStatics.GetPlayerPawn` 0)))
        (bind _returnvalue_location (`KismetMathLibrary.BreakTransform` (`SceneComponent.GetRelativeTransform` (`HSPlayer.Capsule` _asbp_hsplayer))))
        (`KismetSystemLibrary.MoveComponentTo` _scene _returnvalue_location (`SceneComponent.RelativeRotation` _scene) false false 0.1 true)))
    (:`then_1`
      ;[1 1 1] HoverEffect
      (bind _output_get (set `self.SinTimer` (+ (* DeltaSeconds (`self.SpeedHover`)) (`self.SinTimer`))))
      (`SceneComponent.K2_SetWorldLocation` (`self.Scene`) (`KismetMathLibrary.VLerp` (`KismetMathLibrary.MakeVector` _spawnpos_x _spawnpos_y (+ _spawnpos_z _offsetz)) (`KismetMathLibrary.MakeVector` _spawnpos_x _spawnpos_y (- _spawnpos_z _offsetz)) (`KismetMathLibrary.DegSin` _output_get)) false false)
      (`SceneComponent.K2_SetWorldRotation` (`self.Scene`) (`KismetMathLibrary.MakeRotator` (.roll (`self.K2_GetActorRotation`)) (.pitch (`self.K2_GetActorRotation`)) (+ (.yaw (`self.K2_GetActorRotation`)) (* DeltaSeconds (`self.RotationSpeed`)))) false false))))

(fn `UserConstructionScript`
  (set `self.SpawnPos` (`self.K2_GetActorLocation`)))