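; A loot chest actor that holds a resource class and, on taking any damage, spawns that resource at its transform and destroys itself.
; CreateChest stores the resource and derives one of three rarity tiers from a class default, setting a matching custom depth stencil value for each.
; All tiers share one chest mesh and a hard-coded transform.
; Values below the lowest tier only print a German error message.
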(event `self.ReceiveAnyDamage`
  (params (Damage :type "Float (single-precision)") (DamageType :type "DamageType Object Reference") (InstigatedBy :type "Controller Object Reference") (DamageCauser :type "Actor Object Reference"))
  (`|SpawnActorFromClass` (`self.Ressource`) (`self.GetTransform`) "AlwaysSpawn" "OverrideRootScale" null null)
  (`self.K2_DestroyActor`))

(fn `CreateChest`
  (params (Ressource :type "/Game/Gameplay/Resources/Ressources/BP_BaseResouces Class Reference"))
  (bind _staticmesh (`self.StaticMesh`))
  (bind _output_get (set `self.Ressource` Ressource))
  (bind _inventoryindex (defaults `/Game/Gameplay/Resources/BP_Ressource_Base_LoadChest` _output_get))
  (if (> _inventoryindex 5)
    (set `self.Rarity` "NewEnumerator3")
    (`PrimitiveComponent.SetCustomDepthStencilValue` _staticmesh 4)
    (`StaticMeshComponent.SetStaticMesh` _staticmesh "/Game/AncientTreasures/Meshes/SM_Chest_02c.SM_Chest_02c" :!label _label)
    (`self.K2_SetActorTransform` (`KismetMathLibrary.MakeTransform` (240.0 2350.0 0.0) (struct :`Yaw` -90.0) (1.0 1.0 1.0)))
    (elif (> _inventoryindex 3)
      (set `self.Rarity` "NewEnumerator2")
      (`PrimitiveComponent.SetCustomDepthStencilValue` _staticmesh 3)
      (goto _label)
      (elif (> _inventoryindex 1)
        (set `self.Rarity` "NewEnumerator1")
        (`PrimitiveComponent.SetCustomDepthStencilValue` _staticmesh 2)
        (goto _label)
        (else
          (`KismetSystemLibrary.PrintString` "Irgendwas ist schiefgelaufen"))))))

(fn `UserConstructionScript`)