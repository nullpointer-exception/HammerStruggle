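; BP_RessourceBox scatters destructible boxes with a child actor at each one, apparently as resource pickups, and is marked as unused.
; On BeginPlay, Spawn runs Amount times, pairing AddBox with AddRessource.
; AddBox creates a destructible component at a random flat offset scaled by Range and applies Material; AddRessource places a child actor at that same relative location.
; The construction script and Randomize graph are empty.
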(event `self.ReceiveBeginPlay`
  ;[1 1 1] BP by Bea, but not used
  (`self.Spawn`))

(fn `AddBox`
  (returns (RelativeLocation :type "Vector Structure"))
  (bind _returnvalue (`AddComponent|NODE_AddDestructibleComponent-2` :`RelativeTransform` (`KismetMathLibrary.Conv_VectorToTransform` (`KismetMathLibrary.MakeVector` (.x (* (`KismetMathLibrary.RandomUnitVector`) (`self.Range`))) (.y (* (`KismetMathLibrary.RandomUnitVector`) (`self.Range`)))))))
  (`PrimitiveComponent.SetMaterial` _returnvalue 0 (`self.Material`))
  (return (`SceneComponent.RelativeLocation` _returnvalue)))

(fn `AddRessource`
  (params (RelativeLocation :type "Vector Structure"))
  (`AddComponent|NODE_AddChildActorComponent-3` :`RelativeTransform` (`KismetMathLibrary.MakeTransform` RelativeLocation)))

(fn `Spawn`
  (for _ (range 1 (+ (`self.Amount`) 1))
    (bind _relativelocation (`self.AddBox`))
    (`self.AddRessource` _relativelocation)))

(fn `UserConstructionScript`)