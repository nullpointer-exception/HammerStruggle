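; Crystal actor that, once activated through the UI_Well widget, empowers the first BP_AIBase to overlap its sphere.
; Tick polls the widget's flags to close it or arm the crystal, storing one rarity above the selected one, coloring the light and showing the sphere.
; Overlap consumes the charge, scaling the AI's max health, size and damage by rarity, refilling health, assigning a rarity-tiered random resource and blacking out the light.
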(event `self.ReceiveBeginPlay`
  ;[1 1 1] SetPlayer + Disable Sphere
  (`SceneComponent.SetVisibility` (`self.Sphere`) false false)
  (bind _asbp_hsplayer (cast `/Game/Characters/Player/Blueprints/BP_HSPlayer` (`GameplayStatics.GetPlayerPawn` 0)))
  (set `self.PlayerRef` _asbp_hsplayer))

(event `self.ReceiveTick`
  (params (DeltaSeconds :type "Float (single-precision)"))
  (bind _ui_ref (`self.UI_Ref`))
  ;[1 1 1] Check for Activate
  (`/Engine/EditorBlueprintResources/StandardMacros.IsValid` _ui_ref
    (:`Is Valid`
      (`|ExecutionSequence`
        (:`then_0`
          (if (`/Game/UI/CristalUI/UI_Well.IsActive` _ui_ref)
            (`self.SetRarity` (`/Game/UI/CristalUI/UI_Well.CurrRarity` _ui_ref))
            (`self.ToggelLamp` (`self.Loaded Rarity`))
            (`self.CloseUI`)
            (set `/Game/UI/CristalUI/UI_Well.IsActive` false _ui_ref)
            (set `self.Active` true)
            (`SceneComponent.SetVisibility` (`self.Sphere`) true false)))
        (:`then_1`
          (if (`/Game/UI/CristalUI/UI_Well.PressedQuit` _ui_ref)
            (`self.CloseUI`)
            (set `/Game/UI/CristalUI/UI_Well.PressedQuit` false _ui_ref)))))))

(event `self.Sphere.OnComponentBeginOverlap`
  (params (OverlappedComponent :type "PrimitiveComponent Object Reference") (OtherActor :type "Actor Object Reference") (OtherComp :type "PrimitiveComponent Object Reference") (OtherBodyIndex :type Integer) (bFromSweep :type Boolean) (SweepResult :type "HitResult Structure (by ref)"))
  ;[1 1 1] BoostGolem
  (if (`self.Active`)
    (bind _asbp_aibase (cast `/Game/Characters/NPC/Enemies/KI/BP_AIBase` OtherActor))
    (set `self.Active` false)
    (`SceneComponent.SetVisibility` (`self.Sphere`) false false)
    (switch `/Game/Gameplay/Resources/Enum_Rarity` (`self.Loaded Rarity`)
      (:`NewEnumerator1`
        (bind _maxhealth (`/Game/Characters/NPC/Enemies/KI/BP_AIBase.MaxHealth` _asbp_aibase))
        (bind _output_get (set `/Game/Characters/NPC/Enemies/KI/BP_AIBase.Health` (`KismetMathLibrary.Conv_IntToDouble` (`KismetMathLibrary.Round` (* _maxhealth 1.2))) _asbp_aibase))
        (set `/Game/Characters/NPC/Enemies/KI/BP_AIBase.MaxHealth` _output_get _asbp_aibase)
        (`self.SetActorScale3D` _asbp_aibase (1.2 1.2 1.2))
        (bind _ressource (`self.GetRandomRessource` 2))
        (`/Game/Characters/NPC/Enemies/KI/BP_AIBase.SetLoadRessource` _asbp_aibase _ressource)
        (bind _damagemeele (`/Game/Characters/NPC/Enemies/KI/BP_AIBase.DamageMeele` _asbp_aibase))
        (set `/Game/Characters/NPC/Enemies/KI/BP_AIBase.DamageMeele` (`KismetMathLibrary.Conv_IntToDouble` (`KismetMathLibrary.Round` (* _damagemeele 1.2))) _asbp_aibase)
        (bind _damagethrow (`/Game/Characters/NPC/Enemies/KI/BP_AIBase.DamageThrow` _asbp_aibase))
        (set `/Game/Characters/NPC/Enemies/KI/BP_AIBase.DamageThrow` (`KismetMathLibrary.Conv_IntToDouble` (`KismetMathLibrary.Round` (* _damagethrow 1.2))) _asbp_aibase))
      (:`NewEnumerator2`
        (bind _output_get_2 (set `/Game/Characters/NPC/Enemies/KI/BP_AIBase.Health` (`KismetMathLibrary.Conv_IntToDouble` (`KismetMathLibrary.Round` (* _maxhealth 1.4))) _asbp_aibase))
        (set `/Game/Characters/NPC/Enemies/KI/BP_AIBase.MaxHealth` _output_get_2 _asbp_aibase)
        (`self.SetActorScale3D` _asbp_aibase (1.4 1.4 1.4))
        (bind _ressource_2 (`self.GetRandomRessource` 4))
        (`/Game/Characters/NPC/Enemies/KI/BP_AIBase.SetLoadRessource` _asbp_aibase _ressource_2)
        (set `/Game/Characters/NPC/Enemies/KI/BP_AIBase.DamageMeele` (`KismetMathLibrary.Conv_IntToDouble` (`KismetMathLibrary.Round` (* _damagemeele 1.4))) _asbp_aibase)
        (set `/Game/Characters/NPC/Enemies/KI/BP_AIBase.DamageThrow` (`KismetMathLibrary.Conv_IntToDouble` (`KismetMathLibrary.Round` (* _damagethrow 1.4))) _asbp_aibase))
      (:`NewEnumerator3`
        (bind _output_get_3 (set `/Game/Characters/NPC/Enemies/KI/BP_AIBase.Health` (`KismetMathLibrary.Conv_IntToDouble` (`KismetMathLibrary.Round` (* _maxhealth 1.6))) _asbp_aibase))
        (set `/Game/Characters/NPC/Enemies/KI/BP_AIBase.MaxHealth` _output_get_3 _asbp_aibase)
        (`self.SetActorScale3D` _asbp_aibase (1.6 1.6 1.6))
        (bind _ressource_3 (`self.GetRandomRessource` 6))
        (`/Game/Characters/NPC/Enemies/KI/BP_AIBase.SetLoadRessource` _asbp_aibase _ressource_3)
        (set `/Game/Characters/NPC/Enemies/KI/BP_AIBase.DamageMeele` (`KismetMathLibrary.Conv_IntToDouble` (`KismetMathLibrary.Round` (* _damagemeele 1.6))) _asbp_aibase)
        (set `/Game/Characters/NPC/Enemies/KI/BP_AIBase.DamageThrow` (`KismetMathLibrary.Conv_IntToDouble` (`KismetMathLibrary.Round` (* _damagethrow 1.6))) _asbp_aibase)))
    (`LightComponent.SetLightColor` :`self` (`self.PointLight`))))

(fn `CloseUI`
  (bind _returnvalue (`GameplayStatics.GetPlayerController` 0))
  (bind _ui_ref (`self.UI_Ref`))
  (`/Engine/EditorBlueprintResources/StandardMacros.IsValid` _ui_ref
    (:`Is Valid`
      (`Widget.RemoveFromParent` _ui_ref)
      (set `PlayerController.bShowMouseCursor` false _returnvalue)
      (`WidgetBlueprintLibrary.SetInputMode_GameOnly` _returnvalue))))

(fn `GetRandomRessource`
  (params (StartIndex :type Integer))
  (returns (Ressource :type "/Game/Gameplay/Resources/Ressources/BP_BaseResouces Class Reference"))
  (switch `int` (+ StartIndex (`KismetMathLibrary.RandomInteger` 2))
    (:`0`
      (return "/Game/Gameplay/Resources/Ressources/BP_Ressource_Wood.BP_Ressource_Wood_C"))
    (:`1`
      (return "/Game/Gameplay/Resources/Ressources/BP_Ressource_Stone.BP_Ressource_Stone_C"))
    (:`2`
      (return "/Game/Gameplay/Resources/Ressources/BP_Ressource_Iron.BP_Ressource_Iron_C"))
    (:`3`
      (return "/Game/Gameplay/Resources/Ressources/BP_Ressource_Copper.BP_Ressource_Copper_C"))
    (:`4`
      (return "/Game/Gameplay/Resources/Ressources/BP_Ressource_Marbel.BP_Ressource_Marbel_C"))
    (:`5`
      (return "/Game/Gameplay/Resources/Ressources/BP_Ressource_Silver.BP_Ressource_Silver_C"))
    (:`6`
      (return "/Game/Gameplay/Resources/Ressources/BP_Ressource_Gem.BP_Ressource_Gem_C"))
    (:`7`
      (return "/Game/Gameplay/Resources/Ressources/BP_Ressource_Gold.BP_Ressource_Gold_C"))))

(fn `OpenUI`
  (bind _returnvalue (`GameplayStatics.GetPlayerController` 0))
  (bind _ui_ref (`self.UI_Ref`))
  (`/Engine/EditorBlueprintResources/StandardMacros.IsValid` (`self.UI_Ref`)
    (:`Is Valid`
      _)
    (:`Is Not Valid`
      (bind _returnvalue_2 (`|CreateWidget` "/Game/UI/CristalUI/UI_Well.UI_Well_C"))
      (set `self.UI_Ref` _returnvalue_2)))
  (`WidgetBlueprintLibrary.SetInputMode_GameAndUIEx` _returnvalue _ui_ref "DoNotLock" false)
  (set `PlayerController.bShowMouseCursor` true _returnvalue)
  (`UserWidget.AddToViewport` _ui_ref 0))

(fn `SetRarity`
  (params (LoadedRaity :type "/Game/Gameplay/Resources/Enum_Rarity Enum" :default "NewEnumerator0"))
  (switch `/Game/Gameplay/Resources/Enum_Rarity` LoadedRaity
    (:`NewEnumerator0`
      (set `self.Loaded Rarity` "NewEnumerator1"))
    (:`NewEnumerator1`
      (set `self.Loaded Rarity` "NewEnumerator2"))
    (:`NewEnumerator2`
      (set `self.Loaded Rarity` "NewEnumerator3"))))

(fn `ToggelLamp`
  (params (Rarity :type "/Game/Gameplay/Resources/Enum_Rarity Enum" :default "NewEnumerator0"))
  (bind _pointlight (`self.PointLight`))
  (switch `/Game/Gameplay/Resources/Enum_Rarity` Rarity
    (:`NewEnumerator1`
      (`LightComponent.SetLightColor` _pointlight (struct :`G` 0.031802 :`B` 1.0 :`A` 1.0) true))
    (:`NewEnumerator2`
      (`LightComponent.SetLightColor` _pointlight (struct :`R` 0.4375 :`B` 0.393281 :`A` 1.0) true))
    (:`NewEnumerator3`
      (`LightComponent.SetLightColor` _pointlight (struct :`R` 1.0 :`G` 0.831652 :`A` 1.0) true))))

(fn `UserConstructionScript`)