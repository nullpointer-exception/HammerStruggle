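; BP_Chest is a chest Blueprint that opens and closes a UI_Chest widget for player 0.
; ToggelUI creates the widget on first open, caches it in UIRef, and returns it after adding it to the viewport.
; It also switches input mode and cursor visibility to match.
; Tick polls the widget's PressedQuit flag to trigger closing, which removes the widget and resets the flag.
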(event `self.ReceiveTick`
  (params (DeltaSeconds :type "Float (single-precision)"))
  (bind _uiref (`self.UIRef`))
  (`/Engine/EditorBlueprintResources/StandardMacros.IsValid` _uiref
    (:`Is Valid`
      (if (`/Game/UI/ChestUI/UI_Chest.PressedQuit` _uiref)
        (`self.ToggelUI` false)))))

(fn `ToggelUI`
  (params (`Open?` :type Boolean))
  (returns (UiRef :type "UserWidget Object Reference"))
  (bind _returnvalue (`GameplayStatics.GetPlayerController` 0))
  (bind _uiref (`self.UIRef`))
  (bind _uiref_2 (`self.UIRef`))
  (if `Open?`
    (`/Engine/EditorBlueprintResources/StandardMacros.IsValid` _uiref
      (:`Is Valid`
        _)
      (:`Is Not Valid`
        (bind _returnvalue_2 (`|CreateWidget` "/Game/UI/ChestUI/UI_Chest.UI_Chest_C"))
        (set `self.UIRef` _returnvalue_2)))
    (`WidgetBlueprintLibrary.SetInputMode_GameAndUIEx` _returnvalue _uiref_2 "DoNotLock" false)
    (set `PlayerController.bShowMouseCursor` true _returnvalue)
    (`UserWidget.AddToViewport` _uiref_2 0)
    (return _uiref_2)
    (else
      (`/Engine/EditorBlueprintResources/StandardMacros.IsValid` _uiref
        (:`Is Valid`
          (`Widget.RemoveFromParent` _uiref)
          (set `PlayerController.bShowMouseCursor` false _returnvalue)
          (`WidgetBlueprintLibrary.SetInputMode_GameOnly` _returnvalue)
          (set `/Game/UI/ChestUI/UI_Chest.PressedQuit` false _uiref)
          (return null))))))

(fn `UserConstructionScript`)