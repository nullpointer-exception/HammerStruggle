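; Enemy spawner that spawns a batch of AI melee characters once at BeginPlay.
; SpawnEnemy loops over an Amount variable and makes a random two-way pick each pass, though both branches spawn BP_AI_Melee_Character.
; Each spawn takes its transform from SpawnPoint, whose graph holds a random Select among three spawn points that is marked unused.
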(event `self.ReceiveBeginPlay`
  (`self.SpawnEnemy`))

(fn `SpawnEnemy`
  (for _ (range (+ (`self.Amount`) 1))
    (switch `int` (`KismetMathLibrary.RandomIntegerInRange` 0 1)
      (:`0`
        (`|SpawnActorFromClass` "/Game/Characters/NPC/Enemies/KI/Melee/Blueprints/BP_AI_Melee_Character.BP_AI_Melee_Character_C" (`self.SpawnPoint`) "Undefined" "OverrideRootScale" null null))
      (:`1`
        (`|SpawnActorFromClass` "/Game/Characters/NPC/Enemies/KI/Melee/Blueprints/BP_AI_Melee_Character.BP_AI_Melee_Character_C" (`self.SpawnPoint`) "Undefined" "OverrideRootScale" null null)))))

(fn `UserConstructionScript`)